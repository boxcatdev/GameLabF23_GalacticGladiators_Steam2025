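; Voice-over announcer for the GM2 game mode that plays lines for game start, countdown, player death, super star pickup, new leader and collisions.
; It binds to GameMode and FXManager events, then plays cues from VOAudioAtlas on one Speaker, picking new-leader lines by character model.
; ShouldSpeak gates start, death and star lines by playback, cooldown and chance, while the others play ungated.
; The winner-based victory logic is disconnected, so game end is silent.
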(event Custom|OnStartGameVO
  (CallFunction|OnStartGame)
  (for _array_element (Variables|/Game/GameMode2/Programming/Gamemode/GM_GM2.GM_GM2_C|GetPlayers (Variables|Default|GetGameMode))
    (EventDispatchers|BindEventtoOnPlayerKill _array_element (delegate Custom|OnPlayerKillVO))))

(event Custom|OnCountdown
  (CallFunction|Countdown))

(event Custom|OnPlayerKillVO)

(event Custom|OnGameEnd
  (CallFunction|OnEndGame))

(event Custom|OnPlayerDeath
  (params (Player :type PC%20GM2%20Player%20Object%20Reference))
  (CallFunction|OnPlayerKill Player))

(event Custom|SpawnSound
  (params (Sound :type Sound%20Base%20Object%20Reference))
  (bind _speaker (Variables|Default|GetSpeaker))
  (Utilities|IsValid Sound
    (:Is%20Valid
      (Variables|Default|SetCanSpeak false)
      (Audio|Components|Audio|SetSound _speaker Sound)
      (Audio|Components|Audio|Play _speaker 0.0)
      (Utilities|FlowControl|Delay (+ (Variables|/Script/Engine.SoundBase|GetDuration Sound) (Variables|Default|GetDelayBetweenSpeakers)))
      (Variables|Default|SetCanSpeak true))))

(event Custom|OnSuperStarCollect
  (params (Star :type BP%20GM2%20Big%20Star%20Object%20Reference))
  (CallFunction|SuperStarCollect))

(event Custom|OnNewFirstPlace
  (params (Player :type PC%20GM2%20Player%20Object%20Reference))
  (CallFunction|NewFirstPlace Player))

(event Custom|OnPlayerCollision
  (params (Location :type Vector))
  (CallFunction|PlayerCollision))

(event EventBeginPlay
  (bind _gamemode (Variables|Default|GetGameMode))
  (bind _fxmanager (Variables|/Game/GameMode2/Programming/Gamemode/GM_GM2.GM_GM2_C|GetFXManager _gamemode))
  (Utilities|FlowControl|Delay 0.3)
  (CallFunction|GatherVariables)
  (EventDispatchers|BindEventtoOnStartGame _gamemode (delegate Custom|OnStartGameVO))
  (EventDispatchers|AssignGM2GameEnd _fxmanager (delegate Custom|OnGameEnd))
  (EventDispatchers|AssignGM2PlayerDeath _fxmanager (delegate Custom|OnPlayerDeath))
  (EventDispatchers|AssignGM2Countdown _fxmanager (delegate Custom|OnCountdown))
  (EventDispatchers|AssignGM2LargeStarCollected _fxmanager (delegate Custom|OnSuperStarCollect))
  (EventDispatchers|AssignGM2NewFirstPlace _fxmanager (delegate Custom|OnNewFirstPlace))
  (EventDispatchers|AssignGM2PlayerCollision _fxmanager (delegate Custom|OnPlayerCollision)))

(fn ConstructionScript)

(fn GatherVariables
  (bind _asgi_core_game_instance (Utilities|Casting|CastToGI_CORE_GameInstance (Game|GetGameInstance)))
  (Variables|Default|SetGameInstance _asgi_core_game_instance)
  (bind _asgm_gm2 (Utilities|Casting|CastToGM_GM2 (Game|GetGameMode)))
  (Variables|Default|SetGameMode _asgm_gm2))

(fn OnStartGame
  (Utilities|ShouldSpeak
    (:Out
      (bind _soundcue (Default|GetSoundCue (Variables|Default|GetVOAudioAtlas) "NewEnumerator18"))
      (CallFunction|SpawnSound _soundcue))))

(fn OnEndGame)

(fn OnPlayerKill
  (params (KilledPlayer :type PC%20GM2%20Player%20Object%20Reference))
  (Utilities|ShouldSpeak
    (:Out
      (bind _soundcue (Default|GetSoundCue (Variables|Default|GetVOAudioAtlas) "NewEnumerator23"))
      (CallFunction|SpawnSound _soundcue))))

(fn Countdown
  (Audio|Components|Audio|Stop (Variables|Default|GetSpeaker))
  (bind _soundcue (Default|GetSoundCue (Variables|Default|GetVOAudioAtlas) "NewEnumerator53"))
  (CallFunction|SpawnSound _soundcue))

(fn SuperStarCollect
  (Development|PrintString "Super Star Voice Over Called")
  (Utilities|ShouldSpeak
    (:Out
      (bind _soundcue (Default|GetSoundCue (Variables|Default|GetVOAudioAtlas) "NewEnumerator54"))
      (CallFunction|SpawnSound _soundcue))))

(fn NewFirstPlace
  (params (Player :type PC%20GM2%20Player%20Object%20Reference))
  (bind _outenum (Default|GetPlayerModel (Variables|Default|GetGameInstance) (Variables|/Game/GameMode2/Programming/Movement/PC_GM2_Player.PC_GM2_Player_C|GetIndex Player)))
  (bind _output_get (LocalVariables|SetpModel _outenum))
  (switch Utilities|FlowControl|Switch|SwitchonE_PlayerModel _output_get
    (:NewEnumerator4
      (bind _soundcue (Default|GetSoundCue (Variables|Default|GetVOAudioAtlas) "NewEnumerator51"))
      (LocalVariables|SetfinalSoundCue _soundcue))
    (:NewEnumerator0
      (bind _soundcue_2 (Default|GetSoundCue (Variables|Default|GetVOAudioAtlas) "NewEnumerator22"))
      (LocalVariables|SetfinalSoundCue _soundcue_2))
    (:NewEnumerator1
      (bind _soundcue_3 (Default|GetSoundCue (Variables|Default|GetVOAudioAtlas) "NewEnumerator49"))
      (LocalVariables|SetfinalSoundCue _soundcue_3))
    (:NewEnumerator2
      (bind _soundcue_4 (Default|GetSoundCue (Variables|Default|GetVOAudioAtlas) "NewEnumerator50"))
      (LocalVariables|SetfinalSoundCue _soundcue_4)))
  (CallFunction|SpawnSound (LocalVariables|GetfinalSoundCue))
  (Development|PrintText (Utilities|Text|FormatText "NEW FIRST PLACE") true true "(R=1.000000,G=0.334700,B=0.000000,A=1.000000)" 5e+01))

(fn PlayerCollision
  (bind _soundcue (Default|GetSoundCue (Variables|Default|GetVOAudioAtlas) "NewEnumerator24"))
  (CallFunction|SpawnSound _soundcue))