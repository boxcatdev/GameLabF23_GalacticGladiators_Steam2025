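; Announcer voice-over actor for the GM1 game mode, playing 2D lines from the game instance's audio atlas.
; It binds to game mode, FX manager and player events, and polls for players on ice with a looping timer.
; Hit, death, ice and game-end lines pass a ShouldPlay chance and busy check.
; Start, first-place and knockout lines bypass it, the latter two chosen by player model; winner announcement logic is disconnected.
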(event Custom|OnHitVO
  (params (hitBy :type Actor%20Object%20Reference))
  ;[1 1 1] Bind to Player Events
  (CallFunction|OnHit hitBy (stale Custom|OnStartGameVO _array_element)))

(event Custom|OnDieVO
  (params (player :type Actor%20Object%20Reference))
  ;[1 1 1] Bind to Player Events
  (CallFunction|OnDie player))

(event Custom|SpawnSound
  (params (Sound :type Sound%20Base%20Object%20Reference))
  (Variables|Default|SetCanSpeak false)
  (bind _returnvalue (Audio|SpawnSound2D Sound 1.0 1.0 0.0 0))
  (Variables|Default|SetSpeaker _returnvalue)
  (Utilities|FlowControl|Delay (+ (Variables|/Script/Engine.SoundBase|GetDuration Sound) (Variables|Default|GetDelayBetweenAnnouncement)))
  (Variables|Default|SetCanSpeak true))

(event Custom|GM1_GameEnd_Event
  (CallFunction|OnEndGame))

(event Custom|OnStartGameVO
  (bind _gameinstance (Variables|Default|GetGameInstance))
  (bind _gameinstancevariables (Variables|/Game/Core/Programming/Prototypes/GameData/GI_CORE_GameInstance.GI_CORE_GameInstance_C|GetGameInstanceVariables _gameinstance))
  (bind _timebetweenvo (Variables|/Game/Core/Programming/Prototypes/Test_Sai/PDA_GameInstanceSettings.PDA_GameInstanceSettings_C|GetTimeBetweenVO _gameinstancevariables))
  ;[1 1 1] Bind to GameMode Events
  (CallFunction|OnStartGame)
  ;[1 1 1] Get Players
  (Variables|Default|SetPlayers (Variables|/Game/Systems/Blueprints/GM1/Systems/GM_GM1.GM_GM1_C|GetPlayers (Variables|Default|GetGameMode)))
  ;[1 1 1] Bind to Player Events
  (for _array_element (Variables|Default|GetPlayers)
    (EventDispatchers|BindEventtoOnImpulseReceived _array_element (delegate Custom|OnHitVO))
    (Development|PrintString "VO: Bound to On Hit")
    (EventDispatchers|BindEventtoOnDie _array_element (delegate Custom|OnDieVO))
    (Development|PrintString "VO: Bound to On Die"))
  ;[1 1 1] On Ice VO
  (Utilities|Time|SetTimerbyEvent (delegate Custom|OnIceVO) (Math|Random|RandomFloatinRange (.x _timebetweenvo) (.y _timebetweenvo)) true))

(event Custom|OnEndGameVO
  ;[1 1 1] Bind to GameMode Events
  (CallFunction|OnEndGame))

(event Custom|PauseRandomVO
  (params (Duration :type Float%20%28single-precision%29))
  ;[1 1 1] Pause the Random Voice Lines
  (Variables|Default|SetAllowRandomVO false)
  (Utilities|FlowControl|Delay Duration)
  (Variables|Default|SetAllowRandomVO true))

(event Custom|OnIceVO
  ;[1 1 1] On Ice VO
  (Utilities|CheckIce
    (:True
      (CallFunction|OnIce))))

(event Custom|VOEventBindings
  (bind _asgm_gm1 (Utilities|Casting|CastToGM_GM1 (Game|GetGameMode)))
  (EventDispatchers|AssignGM1NewFirstPlace (Variables|/Game/Systems/Blueprints/GM1/Systems/GM_GM1.GM_GM1_C|GetFXManager _asgm_gm1) (delegate Custom|OnNewFirstPlace))
  (EventDispatchers|AssignGM1PlayerDeath (Variables|/Game/Systems/Blueprints/GM1/Systems/GM_GM1.GM_GM1_C|GetFXManager _asgm_gm1) (delegate Custom|GM1_PlayerDeath_Event))
  (EventDispatchers|AssignGM1PlayerRocketBurstImpact (Variables|/Game/Systems/Blueprints/GM1/Systems/GM_GM1.GM_GM1_C|GetFXManager _asgm_gm1) (delegate Custom|GM1_PlayerRocketBurstImpact_Event))
  (EventDispatchers|AssignGM1GameEnd (Variables|/Game/Systems/Blueprints/GM1/Systems/GM_GM1.GM_GM1_C|GetFXManager _asgm_gm1) (delegate Custom|GM1_GameEnd_Event)))

(event Custom|OnNewFirstPlace
  (params (playerId :type Integer))
  (CallFunction|NewFirstPlace playerId))

(event Custom|GM1_PlayerDeath_Event
  (params (player :type BP%20Player%20GM1%20Object%20Reference))
  (CallFunction|PlayerKnockout player))

(event Custom|GM1_PlayerRocketBurstImpact_Event
  (params (player :type BP%20Player%20GM1%20Object%20Reference)))

(event EventBeginPlay
  (Utilities|FlowControl|Delay 0.2)
  ;[1 1 1] Gather Variables
  (bind _asgi_core_game_instance (Utilities|Casting|CastToGI_CORE_GameInstance (Game|GetGameInstance))
    (:then
      (Variables|Default|SetGameInstance _asgi_core_game_instance)
      (bind _asgm_gm1 (Utilities|Casting|CastToGM_GM1 (Game|GetGameMode))
        (:then
          (Variables|Default|SetGameMode _asgm_gm1)
          ;[1 1 1] Bind to GameMode Events
          (EventDispatchers|BindEventtoGameStarted (Variables|Default|GetGameMode) (delegate Custom|OnStartGameVO))
          (EventDispatchers|AssignGM1GameEnd (Variables|/Game/Systems/Blueprints/GM1/Systems/GM_GM1.GM_GM1_C|GetFXManager (Variables|Default|GetGameMode)) (delegate Custom|OnEndGameVO))
          (Variables|Default|SetAudioAtlas (Variables|/Game/Core/Programming/Prototypes/GameData/GI_CORE_GameInstance.GI_CORE_GameInstance_C|GetVOGM1AudioAtlas (Variables|Default|GetGameInstance)))
          (CallFunction|VOEventBindings))
        (:CastFailed
          (Development|PrintString "VO: Cannot find GM_GM1"))))
    (:CastFailed
      (Development|PrintString "VO: cannot find game instance"))))

(event EventTick
  (params (DeltaSeconds :type Float%20%28single-precision%29)))

(fn ConstructionScript)

(fn OnHit
  (params (HitBy :type Actor%20Object%20Reference) (HitPlayer :type Actor%20Object%20Reference))
  (Utilities|ShouldPlay
    (:Out
      (Development|PrintString "VO: On Player Hit")
      (bind _soundcue (Default|GetSoundCue (Variables|Default|GetAudioAtlas) "NewEnumerator11"))
      (bind _returnvalue (Audio|SpawnSound2D _soundcue 1.0 1.0 0.0 0))
      (Variables|Default|SetSpeaker _returnvalue))))

(fn OnDie
  (params (Player :type Actor%20Object%20Reference))
  (Utilities|ShouldPlay
    (:Out
      (Development|PrintString "VO: On Player Die")
      (bind _soundcue (Default|GetSoundCue (Variables|Default|GetAudioAtlas) "NewEnumerator9"))
      (bind _returnvalue (Audio|SpawnSound2D _soundcue 1.0 1.0 0.0 0))
      (Variables|Default|SetSpeaker _returnvalue))))

(fn OnStartGame
  (Development|PrintString "VO: On Start Game")
  (Variables|Default|SetAllowRandomVO true)
  (bind _soundcue (Default|GetSoundCue (Variables|Default|GetAudioAtlas) "NewEnumerator18"))
  (bind _returnvalue (Audio|SpawnSound2D _soundcue 1.0 1.0 0.0 0))
  (Variables|Default|SetSpeaker _returnvalue))

(fn OnEndGame
  (Utilities|ShouldPlay
    (:Out
      (Development|PrintString "VO: On End Game")
      (Variables|Default|SetAllowRandomVO false)
      (bind _soundcue (Default|GetSoundCue (Variables|Default|GetAudioAtlas) "NewEnumerator16"))
      (bind _returnvalue (Audio|SpawnSound2D _soundcue 1.0 1.0 0.0 0))
      (Variables|Default|SetSpeaker _returnvalue)
      (Utilities|Time|SetTimerbyFunctionName 0 "AnnounceWinner" (Variables|/Script/Engine.SoundBase|GetDuration _soundcue)))))

(fn OnIce
  (Utilities|ShouldPlay
    (:Out
      (Development|PrintString "VO: On Player Ice")
      (bind _soundcue (Default|GetSoundCue (Variables|Default|GetAudioAtlas) "NewEnumerator10"))
      (bind _returnvalue (Audio|SpawnSound2D _soundcue 1.0 1.0 0.0 0))
      (Variables|Default|SetSpeaker _returnvalue))))

(fn NewFirstPlace
  (params (PlayerID :type Integer))
  (bind _data (Default|GetPlayerData (Variables|Default|GetGameInstance) PlayerID))
  (switch Utilities|FlowControl|Switch|SwitchonE_PlayerModel (.playermodel _data)
    (:NewEnumerator4
      (bind _soundcue (Default|GetSoundCue (Variables|Default|GetAudioAtlas) "NewEnumerator51"))
      (LocalVariables|SetFinalVO _soundcue))
    (:NewEnumerator0
      (bind _soundcue_2 (Default|GetSoundCue (Variables|Default|GetAudioAtlas) "NewEnumerator52"))
      (LocalVariables|SetFinalVO _soundcue_2))
    (:NewEnumerator1
      (bind _soundcue_3 (Default|GetSoundCue (Variables|Default|GetAudioAtlas) "NewEnumerator49"))
      (LocalVariables|SetFinalVO _soundcue_3))
    (:NewEnumerator2
      (bind _soundcue_4 (Default|GetSoundCue (Variables|Default|GetAudioAtlas) "NewEnumerator50"))
      (LocalVariables|SetFinalVO _soundcue_4)))
  (bind _returnvalue (Audio|SpawnSound2D (LocalVariables|GetFinalVO) 1.0 1.0 0.0 0))
  (Variables|Default|SetSpeaker _returnvalue))

(fn AnnounceWinner)

(fn PlayerKnockout
  (params (Player :type BP%20Player%20GM1%20Object%20Reference))
  (bind _outenum (Default|GetPlayerModel (Variables|Default|GetGameInstance) (Variables|/Game/Systems/Blueprints/GM1/Player/Blueprints/BP_Player_GM1.BP_Player_GM1_C|GetIndex Player)))
  (switch Utilities|FlowControl|Switch|SwitchonE_PlayerModel _outenum
    (:NewEnumerator4
      (bind _soundcue (Default|GetSoundCue (Variables|Default|GetAudioAtlas) "NewEnumerator38"))
      (LocalVariables|SetFinalVO _soundcue))
    (:NewEnumerator0
      (bind _soundcue_2 (Default|GetSoundCue (Variables|Default|GetAudioAtlas) "NewEnumerator37"))
      (LocalVariables|SetFinalVO _soundcue_2))
    (:NewEnumerator1
      (bind _soundcue_3 (Default|GetSoundCue (Variables|Default|GetAudioAtlas) "NewEnumerator35"))
      (LocalVariables|SetFinalVO _soundcue_3))
    (:NewEnumerator2
      (bind _soundcue_4 (Default|GetSoundCue (Variables|Default|GetAudioAtlas) "NewEnumerator36"))
      (LocalVariables|SetFinalVO _soundcue_4)))
  (bind _returnvalue (Audio|SpawnSound2D (LocalVariables|GetFinalVO) 1.0 1.0 0.0 0))
  (Variables|Default|SetSpeaker _returnvalue))

(fn PlayerHit
  (params (Player :type BP%20Player%20GM1%20Object%20Reference))
  (bind _soundcue (Default|GetSoundCue (Variables|Default|GetAudioAtlas) "NewEnumerator11"))
  (CallFunction|SpawnSound _soundcue))