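; Prototype sound effects manager for the GM1 game mode, playing audio for players, hazards, the crown and match events.
; After a short BeginPlay delay, it binds handlers to the GM_GM1 FXManager's events.
; Handlers play AudioAtlas cues at actor locations or in 2D, with burst impacts adding a per-character-model sound.
; Running only prints a placeholder, wall drops are unhandled, and the graph's AudioAtlas assignment is disconnected.
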(event Custom|PlayerEventBinding
  (bind _gamemode (Variables|References|GetGameMode))
  (bind _fxmanager (Variables|/Game/Systems/Blueprints/GM1/Systems/GM_GM1.GM_GM1_C|GetFXManager _gamemode))
  ;[1 1 1] i don't know what's real anymore
  (EventDispatchers|BindEventtoGM1PlayerRocketBurstStarted _fxmanager (delegate Custom|OnRocketBurstStarted))
  (EventDispatchers|BindEventtoGM1PlayerRocketBurstImpact _fxmanager (delegate Custom|OnRocketBurstImpact))
  (EventDispatchers|BindEventtoGM1PlayerRocketBurstRecharged _fxmanager (delegate Custom|OnRocketBurstRecharged))
  (EventDispatchers|BindEventtoGM1PlayerDeath _fxmanager (delegate Custom|OnPlayerDeath))
  (EventDispatchers|BindEventtoGM1PlayerSpawn _fxmanager (delegate Custom|OnPlayerSpawn))
  (EventDispatchers|BindEventtoGM1PlayerRunning _fxmanager (delegate Custom|OnPlayerRunning)))

(event Custom|HazardEventBinding
  (bind _gamemode (Variables|References|GetGameMode))
  (bind _fxmanager (Variables|/Game/Systems/Blueprints/GM1/Systems/GM_GM1.GM_GM1_C|GetFXManager _gamemode))
  ;[1 1 1] i don't know what's real anymore
  (EventDispatchers|BindEventtoGM1HazardBumpersCollision _fxmanager (delegate Custom|OnHazardBumpersCollision))
  (EventDispatchers|BindEventtoGM1HazardBumpersLower _fxmanager (delegate Custom|OnHazardBumpersLower))
  (EventDispatchers|BindEventtoGM1HazardBumpersRaise _fxmanager (delegate Custom|OnHazardBumpersRaise))
  (EventDispatchers|BindEventtoGM1HazardIceSpreading _fxmanager (delegate Custom|OnHazardIceSpreading))
  (EventDispatchers|BindEventtoGM1HazardMeteorImpact _fxmanager (delegate Custom|OnHazardMeteorImpact))
  (EventDispatchers|BindEventtoGM1HazardMeteorSpawn _fxmanager (delegate Custom|OnHazardMeteorSpawn))
  (EventDispatchers|BindEventtoGM1HazardMeteorTarget _fxmanager (delegate Custom|OnHazardMeteorTarget))
  (EventDispatchers|BindEventtoGM1HazardSpawnAlert _fxmanager (delegate Custom|OnHazardSpawnAlert))
  (EventDispatchers|BindEventtoGM1HazardLargeMeteorImpact _fxmanager (delegate Custom|OnLargeMeteorImpact))
  (EventDispatchers|BindEventtoGM1HazardLargeMeteorSpawn _fxmanager (delegate Custom|OnLargeMeteorSpawn))
  (EventDispatchers|BindEventtoGM1HazardLargeMeteorTarget _fxmanager (delegate Custom|OnLargeMeteorTarget))
  (EventDispatchers|AssignGM1WallsRemoved _fxmanager (delegate Custom|OnWallsDropped)))

(event Custom|OnHazardBumpersCollision
  (params (bumper :type BP%20Bumper%20Object%20Reference) (player :type BP%20Player%20GM1%20Object%20Reference))
  ;[1 1 1] i don't know what's real anymore
  (HazardEvents|HazardBumpersCollision bumper player))

(event Custom|OnCrownPreSpawn
  (params (crown :type BP%20Crown%20Object%20Reference))
  ;[1 1 1] i don't know what's real anymore
  (CrownEvents|CrownPreSpawn crown))

(event Custom|OnCrownSpawn
  (params (crown :type BP%20Crown%20Object%20Reference))
  ;[1 1 1] i don't know what's real anymore
  (CrownEvents|CrownSpawn crown))

(event Custom|OnCrownPickup
  (params (crown :type BP%20Crown%20Object%20Reference) (newOwner :type BP%20Player%20GM1%20Object%20Reference))
  ;[1 1 1] i don't know what's real anymore
  (CrownEvents|CrownPickup crown newOwner))

(event Custom|OnCrownStolen
  (params (crown :type BP%20Crown%20Object%20Reference) (newOwner :type BP%20Player%20GM1%20Object%20Reference) (oldOwner :type BP%20Player%20GM1%20Object%20Reference))
  ;[1 1 1] i don't know what's real anymore
  (CrownEvents|CrownStolen crown newOwner oldOwner))

(event Custom|OnHazardBumpersRaise
  (params (bumper :type BP%20Bumper%20Object%20Reference))
  ;[1 1 1] i don't know what's real anymore
  (HazardEvents|HazardBumpersRaise bumper))

(event Custom|OnHazardIceSpreading
  (params (isSpreading :type Boolean))
  ;[1 1 1] i don't know what's real anymore
  (HazardEvents|HazardIceSpreading isSpreading))

(event Custom|OnHazardMeteorImpact
  (params (meteor :type BP%20GM1%20Meteor%20Object%20Reference) (location :type Vector))
  ;[1 1 1] i don't know what's real anymore
  (HazardEvents|HazardMeteorImpact meteor))

(event Custom|OnHazardMeteorSpawn
  (params (meteor :type BP%20GM1%20Meteor%20Object%20Reference))
  ;[1 1 1] i don't know what's real anymore
  (HazardEvents|HazardMeteorSpawn meteor))

(event Custom|OnHazardMeteorTarget
  (params (AOEZone :type BP%20GM1%20AOE%20Zone%20Object%20Reference))
  ;[1 1 1] i don't know what's real anymore
  (HazardEvents|HazardMeteorTarget AOEZone))

(event Custom|CrownEventBinding
  (bind _gamemode (Variables|References|GetGameMode))
  (bind _fxmanager (Variables|/Game/Systems/Blueprints/GM1/Systems/GM_GM1.GM_GM1_C|GetFXManager _gamemode))
  ;[1 1 1] i don't know what's real anymore
  (EventDispatchers|BindEventtoGM1CrownPreSpawn _fxmanager (delegate Custom|OnCrownPreSpawn))
  (EventDispatchers|BindEventtoGM1CrownSpawn _fxmanager (delegate Custom|OnCrownSpawn))
  (EventDispatchers|BindEventtoGM1CrownPickedUp _fxmanager (delegate Custom|OnCrownPickup))
  (EventDispatchers|BindEventtoGM1CrownStolen _fxmanager (delegate Custom|OnCrownStolen)))

(event Custom|OnHazardSpawnAlert
  ;[1 1 1] i don't know what's real anymore
  (HazardEvents|HazardSpawnAlert))

(event Custom|OnLargeMeteorImpact
  (params (meteor :type BP%20GM1%20Meteor%20Object%20Reference) (NewParam :type Vector))
  ;[1 1 1] i don't know what's real anymore
  (CallFunction|OnHazardMeteorImpact meteor "0, 0, 0"))

(event Custom|OnLargeMeteorSpawn
  (params (meteor :type BP%20GM1%20Meteor%20Object%20Reference))
  ;[1 1 1] i don't know what's real anymore
  (CallFunction|OnHazardMeteorSpawn meteor))

(event Custom|OnLargeMeteorTarget
  (params (AOEZone :type BP%20GM1%20AOE%20Zone%20Object%20Reference))
  ;[1 1 1] i don't know what's real anymore
  (CallFunction|OnHazardMeteorTarget AOEZone))

(event Custom|OnWallsDropped
  (params (walls :type Array%20of%20Skeletal%20Mesh%20Actor%20Object%20References))
  ;[1 1 1] i don't know what's real anymore
)

(event Custom|GameModeEventBinding
  (bind _gamemode (Variables|References|GetGameMode))
  (bind _fxmanager (Variables|/Game/Systems/Blueprints/GM1/Systems/GM_GM1.GM_GM1_C|GetFXManager _gamemode))
  (EventDispatchers|AssignGM1Countdown _fxmanager (delegate Custom|OnGameModeCountdown))
  (EventDispatchers|AssignGM1TenSecondsLeft _fxmanager (delegate Custom|OnGameModeTenSecondsLeft))
  (EventDispatchers|AssignGM1IntroCutscene _fxmanager (delegate Custom|OnGameModeIntroCutscene))
  (EventDispatchers|AssignGM1GameEnd _fxmanager (delegate Custom|OnGameModeGameEnd))
  (EventDispatchers|AssignGM1GameStart _fxmanager (delegate Custom|GM1_GameStart_Event)))

(event Custom|OnGameModeCountdown
  (params (elapsed :type Float%20%28double-precision%29) (remaining :type Float%20%28double-precision%29))
  (CallFunction|GameModeCutsceneCountdown))

(event Custom|OnGameModeTenSecondsLeft
  (CallFunction|GameModeTenSecondsLeft))

(event Custom|OnGameModeIntroCutscene
  (CallFunction|GameModeIntroCutscene))

(event Custom|OnGameModeGameEnd
  (CallFunction|GameModeGameEnd))

(event Custom|OnHazardBumpersLower
  (params (bumper :type BP%20Bumper%20Object%20Reference))
  ;[1 1 1] i don't know what's real anymore
  (HazardEvents|HazardBumpersLower bumper))

(event Custom|GM1_GameStart_Event
  (CallFunction|GameModeGameStart))

(event Custom|OnRocketBurstStarted
  (params (player :type BP%20Player%20GM1%20Object%20Reference))
  ;[1 1 1] i don't know what's real anymore
  (PlayerEvents|RocketBurstStarted player))

(event Custom|OnRocketBurstImpact
  (params (player :type BP%20Player%20GM1%20Object%20Reference) (location :type Vector))
  ;[1 1 1] i don't know what's real anymore
  (PlayerEvents|RocketBurstImpact player))

(event Custom|OnRocketBurstRecharged
  (params (player :type BP%20Player%20GM1%20Object%20Reference))
  ;[1 1 1] i don't know what's real anymore
  (PlayerEvents|RocketBurstRecharged player))

(event Custom|OnPlayerDeath
  (params (player :type BP%20Player%20GM1%20Object%20Reference))
  ;[1 1 1] i don't know what's real anymore
  (PlayerEvents|PlayerDeath player))

(event Custom|OnPlayerSpawn
  (params (player :type BP%20Player%20GM1%20Object%20Reference))
  ;[1 1 1] i don't know what's real anymore
  (PlayerEvents|PlayerSpawn player))

(event Custom|OnPlayerRunning
  (params (state :type Boolean) (player :type BP%20Player%20GM1%20Object%20Reference))
  ;[1 1 1] i don't know what's real anymore
  (PlayerEvents|PlayerRunning state player))

(event EventBeginPlay
  (Utilities|FlowControl|Delay 0.5)
  ;[1 1 1] Gather Variables
  (bind _asgm_gm1 (Utilities|Casting|CastToGM_GM1 (Game|GetGameMode)))
  (Variables|References|SetGameMode _asgm_gm1)
  (CallFunction|PlayerEventBinding)
  (CallFunction|HazardEventBinding)
  (CallFunction|CrownEventBinding)
  (CallFunction|GameModeEventBinding))

(fn ConstructionScript)

(fn RocketBurstStarted
  (params (Player :type BP%20Player%20GM1%20Object%20Reference))
  (bind _sound_cue (Default|GetSoundCue (Variables|References|GetAudioAtlas) "NewEnumerator15" true))
  (Audio|PlaySoundatLocation _sound_cue (Transformation|GetActorLocation Player) "0, 0, 0" 1.0 1.0 0.0 0 0 0 0))

(fn RocketBurstImpact
  (params (Player :type BP%20Player%20GM1%20Object%20Reference))
  (bind _returnvalue (Transformation|GetActorLocation Player))
  (bind _sound_cue (Default|GetSoundCue (Variables|References|GetAudioAtlas) "NewEnumerator16" true))
  (Audio|PlaySoundatLocation _sound_cue _returnvalue "0, 0, 0" 1.0 1.0 0.0 0 0 0 0)
  (bind _asgi_core_game_instance (Utilities|Casting|CastToGI_CORE_GameInstance (Game|GetGameInstance)))
  (bind _outenum (Default|GetPlayerModel _asgi_core_game_instance (Variables|/Game/Systems/Blueprints/GM1/Player/Blueprints/BP_Player_GM1.BP_Player_GM1_C|GetIndex Player)))
  (switch Utilities|FlowControl|Switch|SwitchonE_PlayerModel _outenum
    (:NewEnumerator4
      (bind _sound_cue_2 (Default|GetSoundCue (Variables|References|GetAudioAtlas) "NewEnumerator41" false))
      (LocalVariables|SetFinalSFX _sound_cue_2))
    (:NewEnumerator0
      (bind _sound_cue_3 (Default|GetSoundCue (Variables|References|GetAudioAtlas) "NewEnumerator42" false))
      (LocalVariables|SetFinalSFX _sound_cue_3))
    (:NewEnumerator1
      (bind _sound_cue_4 (Default|GetSoundCue (Variables|References|GetAudioAtlas) "NewEnumerator39" false))
      (LocalVariables|SetFinalSFX _sound_cue_4))
    (:NewEnumerator2
      (bind _sound_cue_5 (Default|GetSoundCue (Variables|References|GetAudioAtlas) "NewEnumerator40" false))
      (LocalVariables|SetFinalSFX _sound_cue_5)))
  (Audio|PlaySoundatLocation (LocalVariables|GetFinalSFX) _returnvalue "0, 0, 0" 1.0 1.0 0.0 0 0 0 0))

(fn RocketBurstRecharged
  (params (Player :type BP%20Player%20GM1%20Object%20Reference))
  (bind _sound_cue (Default|GetSoundCue (Variables|References|GetAudioAtlas) "NewEnumerator17" true))
  (Audio|PlaySoundatLocation _sound_cue (Transformation|GetActorLocation Player) "0, 0, 0" 1.0 1.0 0.0 0 0 0 0))

(fn PlayerDeath
  (params (Player :type BP%20Player%20GM1%20Object%20Reference))
  (bind _sound_cue (Default|GetSoundCue (Variables|References|GetAudioAtlas) "NewEnumerator18" true))
  (Audio|PlaySoundatLocation _sound_cue (Transformation|GetActorLocation Player) "0, 0, 0" 1.0 1.0 0.0 0 0 0 0))

(fn PlayerSpawn
  (params (Player :type BP%20Player%20GM1%20Object%20Reference))
  (bind _sound_cue (Default|GetSoundCue (Variables|References|GetAudioAtlas) "NewEnumerator19" true))
  (Audio|PlaySoundatLocation _sound_cue (Transformation|GetActorLocation Player) "0, 0, 0" 1.0 1.0 0.0 0 0 0 0))

(fn PlayerRunning
  (params (State :type Boolean) (Player :type BP%20Player%20GM1%20Object%20Reference))
  (if State
    (Development|PrintString (Utilities|String|Append "[" (Utilities|GetDisplayName Player) "] Footstep sound are not working yet sorryyy!!!!") true true "(R=1.000000,G=0.093211,B=0.123059,A=1.000000)")))

(fn HazardBumpersCollision
  (params (Bumpers :type BP%20Bumper%20Object%20Reference) (Player :type BP%20Player%20GM1%20Object%20Reference))
  (bind _sound_cue (Default|GetSoundCue (Variables|References|GetAudioAtlas) "NewEnumerator28" true))
  (Audio|PlaySoundatLocation _sound_cue (Transformation|GetActorLocation Bumpers) "0, 0, 0" 1.0 1.0 0.0 0 0 0 0))

(fn HazardBumpersLower
  (params (Bumper :type BP%20Bumper%20Object%20Reference))
  (bind _sound_cue (Default|GetSoundCue (Variables|References|GetAudioAtlas) "NewEnumerator29" true))
  (Audio|PlaySoundatLocation _sound_cue (Transformation|GetActorLocation Bumper) "0, 0, 0" 1.0 1.0 0.0 0 0 0 0))

(fn HazardBumpersRaise
  (params (Bumper :type BP%20Bumper%20Object%20Reference))
  (bind _sound_cue (Default|GetSoundCue (Variables|References|GetAudioAtlas) "NewEnumerator26" true))
  (Audio|PlaySoundatLocation _sound_cue (Transformation|GetActorLocation Bumper) "0, 0, 0" 1.0 1.0 0.0 0 0 0 0))

(fn HazardIceSpreading
  (params (Is%20Spreading :type Boolean))
  (if Is%20Spreading
    (bind _sound_cue (Default|GetSoundCue (Variables|References|GetAudioAtlas) "NewEnumerator25" true))
    (Audio|PlaySound2D _sound_cue 1.0 1.0 0.0 0 0)))

(fn HazardMeteorImpact
  (params (Meteor :type BP%20GM1%20Meteor%20Object%20Reference))
  (bind _sound_cue (Default|GetSoundCue (Variables|References|GetAudioAtlas) "NewEnumerator46" true))
  (Audio|PlaySoundatLocation _sound_cue (Transformation|GetActorLocation Meteor) "0, 0, 0" 1.0 1.0 0.0 0 0 0 0))

(fn HazardMeteorSpawn
  (params (Meteor :type BP%20GM1%20Meteor%20Object%20Reference))
  (bind _sound_cue (Default|GetSoundCue (Variables|References|GetAudioAtlas) "NewEnumerator21" true))
  (Audio|PlaySoundatLocation _sound_cue (Transformation|GetActorLocation Meteor) "0, 0, 0" 1.0 1.0 0.0 0 0 0 0))

(fn HazardMeteorTarget
  (params (AOEZone :type BP%20GM1%20AOE%20Zone%20Object%20Reference))
  (bind _sound_cue (Default|GetSoundCue (Variables|References|GetAudioAtlas) "NewEnumerator21" true))
  (Audio|PlaySoundatLocation _sound_cue (Transformation|GetActorLocation AOEZone) "0, 0, 0" 1.0 1.0 0.0 0 0 0 0))

(fn HazardSpawnAlert
  (bind _sound_cue (Default|GetSoundCue (Variables|References|GetAudioAtlas) "NewEnumerator38" true))
  (Audio|PlaySound2D _sound_cue 1.0 1.0 0.0 0 0))

(fn CrownPreSpawn
  (params (Crown :type BP%20Crown%20Object%20Reference))
  (bind _sound_cue (Default|GetSoundCue (Variables|References|GetAudioAtlas) "NewEnumerator11" true))
  (Audio|PlaySoundatLocation _sound_cue (Transformation|GetActorLocation Crown) "0, 0, 0" 1.0 1.0 0.0 0 0 0 0))

(fn CrownSpawn
  (params (Crown :type BP%20Crown%20Object%20Reference))
  (bind _sound_cue (Default|GetSoundCue (Variables|References|GetAudioAtlas) "NewEnumerator30" true))
  (Audio|PlaySoundatLocation _sound_cue (Transformation|GetActorLocation Crown) "0, 0, 0" 1.0 1.0 0.0 0 0 0 0))

(fn CrownPickup
  (params (Crown :type BP%20Crown%20Object%20Reference) (NewOwner :type BP%20Player%20GM1%20Object%20Reference))
  (bind _sound_cue (Default|GetSoundCue (Variables|References|GetAudioAtlas) "NewEnumerator32" true))
  (Audio|PlaySoundatLocation _sound_cue (Transformation|GetActorLocation NewOwner) "0, 0, 0" 1.0 1.0 0.0 0 0 0 0))

(fn CrownStolen
  (params (Crown :type BP%20Crown%20Object%20Reference) (New%20Owner :type BP%20Player%20GM1%20Object%20Reference) (Old%20Owner :type BP%20Player%20GM1%20Object%20Reference))
  (bind _asgi_core_game_instance (Utilities|Casting|CastToGI_CORE_GameInstance (Game|GetGameInstance)))
  (bind _sound_cue (Default|GetSoundCue (Variables|/Game/Core/Programming/Prototypes/GameData/GI_CORE_GameInstance.GI_CORE_GameInstance_C|GetSFXGM1AudioAtlas _asgi_core_game_instance) "NewEnumerator31" false))
  (Utilities|IsValid _sound_cue
    (:Is%20Valid
      (Audio|PlaySound2D _sound_cue 7.0 1.0 0.0 0 0))))

(fn HazardWallsDropped
  (params (Walls :type Array%20of%20Static%20Mesh%20Actor%20Object%20References))
  (for _array_element Walls
    (bind _sound_cue (Default|GetSoundCue (Variables|References|GetAudioAtlas) "NewEnumerator29" false))
    (Audio|PlaySoundatLocation _sound_cue (Transformation|GetActorLocation _array_element) "0, 0, 0" 1.0 1.0 0.0 0 0 0 0)))

(fn GameModeCutsceneCountdown
  (bind _sound_cue (Default|GetSoundCue (Variables|References|GetAudioAtlas) "NewEnumerator33" false))
  (Audio|PlaySound2D _sound_cue 1.0 1.0 0.0 0 0))

(fn GameModeTenSecondsLeft
  (bind _sound_cue (Default|GetSoundCue (Variables|References|GetAudioAtlas) "NewEnumerator36" false))
  (Audio|PlaySound2D _sound_cue 1.0 1.0 0.0 0 0))

(fn GameModeIntroCutscene
  (Development|PrintString "UIIntroCutscene" true true "(R=1.000000,G=0.731559,B=0.179725,A=1.000000)" 1e+02)
  (bind _sound_cue (Default|GetSoundCue (Variables|References|GetAudioAtlas) "NewEnumerator48" false))
  (Audio|PlaySound2D _sound_cue 1.0 1.0 0.0 0 0))

(fn GameModeGameEnd
  (bind _sound_cue (Default|GetSoundCue (Variables|References|GetAudioAtlas) "NewEnumerator37" false))
  (Audio|PlaySound2D _sound_cue 1.0 1.0 0.0 0 0))

(fn GameModeGameStart
  (bind _sound_cue (Default|GetSoundCue (Variables|References|GetAudioAtlas) "NewEnumerator34" false))
  (Audio|PlaySound2D _sound_cue 1.0 1.0 0.0 0 0))