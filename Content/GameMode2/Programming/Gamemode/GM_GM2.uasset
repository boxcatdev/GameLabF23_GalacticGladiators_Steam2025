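; Game mode for GM2 that runs a timed local-multiplayer round from intro to results.
; BeginPlay spawns players from game instance data, or one as fallback, on a shared camera, then runs a skippable intro sequence and countdown before starting play and HUD.
; Timers cue end-of-round FX through BP_FXEventManager.
; At time-up it saves scores to the game instance, shows the lowest scorer as winner and opens the results level.
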(event Custom|Begin%20Time%20Limit%20Objective
  (bind _objective (Variables|References|GetObjective))
  (bind _round_length (Variables|/Game/GameMode2/Programming/Gamemode/DA_GM2_Objective.DA_GM2_Objective_C|GetRound%20Length _objective))
  (Utilities|Time|SetTimerbyEvent (delegate Custom|TenSecondsSFX) (- _round_length 1e+01))
  (Utilities|Time|SetTimerbyEvent (delegate Custom|Countdown) (- _round_length 5.0))
  (Utilities|FlowControl|Delay (Variables|/Game/GameMode2/Programming/Gamemode/DA_GM2_Objective.DA_GM2_Objective_C|GetRound%20Length (Variables|References|GetObjective)))
  (CallFunction|EndGame))

(event Custom|TenSecondsSFX
  (Default|CallGM2TenSecondsLeft (Variables|Default|GetFXManager)))

(event Custom|Countdown
  (Default|CallGM2Countdown (Variables|Default|GetFXManager)))

(event Custom|IntroAnim
  ;[0.1479 1 0] Intro Animation Cutscene
  (if (not (Variables|Default|GetPlayingCutscene))
    (Variables|Default|SetPlayingCutscene true)
    (bind _returnvalue (Actor|GetActorOfClass "/Script/LevelSequence.LevelSequenceActor"))
    (Utilities|IsValid _returnvalue
      (:Is%20Valid
        (Sequencer|Player|Play (Variables|/Script/LevelSequence.LevelSequenceActor|GetSequencePlayer _returnvalue) :!class /Script/MovieScene.MovieSceneSequencePlayer)
        (EventDispatchers|BindEventtoOnStop (Variables|/Script/LevelSequence.LevelSequenceActor|GetSequencePlayer _returnvalue) (delegate Custom|OnCutsceneEnd))
        (Development|PrintString (Utilities|String|ToString(Float) (Class|TimeManagementBlueprintLibrary|ToSeconds(QualifiedFrameTime) (Media|MediaPlayer|GetDuration (Variables|/Script/LevelSequence.LevelSequenceActor|GetSequencePlayer _returnvalue)))) true true "(R=0.000000,G=0.660000,B=1.000000,A=1.000000)" (Class|TimeManagementBlueprintLibrary|ToSeconds(QualifiedFrameTime) (Media|MediaPlayer|GetDuration (Variables|/Script/LevelSequence.LevelSequenceActor|GetSequencePlayer _returnvalue))))
        (Development|PrintString "Intro Anim Duration")
        (Variables|Default|SetCutsceneDuration (Class|TimeManagementBlueprintLibrary|ToSeconds(QualifiedFrameTime) (Media|MediaPlayer|GetDuration (Variables|/Script/LevelSequence.LevelSequenceActor|GetSequencePlayer _returnvalue))))))))

(event Custom|OnCutsceneEnd
  (if (Variables|Default|GetPlayingCutscene)
    (Variables|Default|SetPlayingCutscene false)
    (Actor|GetActorOfClass "/Script/Engine.CameraActor")
    (Development|PrintString "[CUTSCENE] Cutscene Over" true true "(R=1.000000,G=0.070588,B=0.450980,A=1.000000)")
    (Default|CallOnCutsceneEnded)))

(event Custom|PauseForCountdown
  (params (NewParam :type Boolean)))

(event Custom|SkipCutscene
  ;[0.1479 1 0] Intro Animation Cutscene
  ;;[0.1349 1 0] Skipped Cutscene
  (if (Variables|Default|GetPlayingCutscene)
    (Utilities|IsValid (Variables|/Script/LevelSequence.LevelSequenceActor|GetSequencePlayer (stale Custom|IntroAnim _returnvalue))
      (:Is%20Valid
        (Class|MovieSceneSequencePlayer|GotoEndandStop (Variables|/Script/LevelSequence.LevelSequenceActor|GetSequencePlayer (stale Custom|IntroAnim _returnvalue)))
        (Development|PrintString "Skipped Cutscene")))))

(event Custom|EndGame
  (CallFunction|SavePlayerScores)
  ;[1 1 1] Show the winner
  (CallFunction|ShowWinner)
  (Development|PrintText "Game Ended" true true "(R=0.284255,G=1.000000,B=0.136735,A=1.000000)")
  (bind _asgi_core_game_instance (Utilities|Casting|CastToGI_CORE_GameInstance (Game|GetGameInstance)))
  (Default|PlayMusic _asgi_core_game_instance "NewEnumerator3" 0.0)
  (Default|CallOnEndGame)
  (Development|PrintString "[ANNOUNCE WINNER]" true true "(R=1.000000,G=0.747086,B=0.100902,A=1.000000)" 5e+01)
  (Default|CallGM2GameEnd (Variables|Default|GetFXManager))
  (Utilities|Time|SetTimerbyEvent (delegate Custom|GoToNextLevelEvent) 4.0))

(event Custom|GoToNextLevelEvent
  (Development|PrintString "GoToNextLevel")
  (CallFunction|GotoNextLevel))

(event EventBeginPlay
  (bind _objective (Variables|References|GetObjective))
  (bind _pregame_countdown_length (Variables|/Game/GameMode2/Programming/Gamemode/DA_GM2_Objective.DA_GM2_Objective_C|GetPregame%20Countdown%20Length _objective))
  (bind _returnvalue (Actor|GetActorOfClass "/Game/Systems/Blueprints/BP_FXEventManager.BP_FXEventManager_C"))
  (Variables|Default|SetFXManager _returnvalue)
  (bind _failed (CallFunction|CacheGlobals))
  (if _failed
    (CallFunction|SpawnPlayer (Utilities|Array|Get(acopy) (Variables|PlayerData|GetPlayerStarts)))
    (else
      ;[1 1 1] Play the game
      (CallFunction|SpawnPlayersfromGameInstance)))
  (Utilities|FlowControl|Delay 0.2)
  (CallFunction|IntroAnim)
  (bind _asgi_core_game_instance (Utilities|Casting|CastToGI_CORE_GameInstance (Game|GetGameInstance)))
  (bind _soundcue (Default|GetSoundCue (Variables|/Game/Core/Programming/Prototypes/GameData/GI_CORE_GameInstance.GI_CORE_GameInstance_C|GetSFXGM2AudioAtlas _asgi_core_game_instance) "NewEnumerator39" false))
  (Audio|PlaySound2D _soundcue 1.0 1.0 0.0 0 0)
  (bind _returnvalue_2 (UserInterface|CreateWidget "/Game/Core/Programming/Prototypes/Test_Sai/WBP_CutsceneSkip.WBP_CutsceneSkip_C"))
  (UserInterface|Viewport|AddtoViewport _returnvalue_2 0)
  (Utilities|FlowControl|Delay (Variables|Default|GetCutsceneDuration))
  (Widget|RemovefromParent _returnvalue_2)
  (bind _returnvalue_3 (UserInterface|CreateWidget "/Game/Core/Programming/Prototypes/Test_Ryan/Widgets/WBP_Core_PregameCountdown.WBP_Core_PregameCountdown_C" 0 (Math|Float|Truncate _pregame_countdown_length)))
  (UserInterface|Viewport|AddtoViewport _returnvalue_3 0)
  (Utilities|FlowControl|Delay _pregame_countdown_length)
  (Development|PrintString "[COUNTDOWN] Ended" true true "(R=1.000000,G=0.070588,B=0.450980,A=1.000000)")
  (Default|CallOnCountdownEnded)
  (CallFunction|StartGame)
  (CallFunction|InitializeHUD))

(event EventHandleStartingNewPlayer
  (params (NewPlayer :type Player%20Controller%20Object%20Reference))
  ;[1 1 1] Possible Work Around
  (|CallParentFunction NewPlayer)
  (Input|AddMappingContext (PlayerController|LocalPlayerSubsystems|GetEnhancedInputLocalPlayerSubsystem NewPlayer) "/Game/GameMode2/Design/Input/IMC_GM2_Default.IMC_GM2_Default" 0 "(bIgnoreAllPressedKeysUntilRelease=True,bForceImmediately=False)"))

(fn ConstructionScript)

(fn SpawnInputRecievers
  (bind _returnvalue (Class|GameplayStatics|GetPlayerControllerfromID))
  (for (_ _array_index) (Variables|PlayerData|GetPlayerStarts)
    (LocalVariables|SetIndex _array_index)
    ;[0 0 0 0.5] Setup Local Players and Assign IMCs
    (bind _returnvalue_2 (Class|GameplayStatics|CreatePlayer (LocalVariables|GetIndex))) ; -1 Auto Increment doesn't work in UE5 :D
    (if (> (LocalVariables|GetIndex) 0)
      ;[0 0 0 0.5] Spawn Input Recievers
      (Input|AddMappingContext (PlayerController|LocalPlayerSubsystems|GetEnhancedInputLocalPlayerSubsystem _returnvalue_2) "/Game/GameMode2/Design/Input/IMC_GM2_Default.IMC_GM2_Default" 0 "(bIgnoreAllPressedKeysUntilRelease=True,bForceImmediately=False)")
      (bind _returnvalue_3 (Game|SpawnActorfromClass "/Game/GameMode2/Programming/Gamemode/BP_GM2_InputReciever.BP_GM2_InputReciever_C" (Transformation|GetActorTransform (Utilities|Array|Get(acopy) (Variables|PlayerData|GetPlayerStarts) (LocalVariables|GetIndex))) "Undefined" "MultiplyWithRoot" 0 (LocalVariables|GetIndex) 0))
      ;[0 0 0 0.5] Possess Pawn
      (Utilities|Array|AddUnique (Variables|PlayerData|GetPlayerInputRecievers) _returnvalue_3)
      (Pawn|Possess (Class|GameplayStatics|GetPlayerControllerfromID (LocalVariables|GetIndex)) _returnvalue_3)
      (Utilities|Array|AddUnique (Variables|PlayerData|GetPlayerControllers) (Class|GameplayStatics|GetPlayerControllerfromID (LocalVariables|GetIndex)))
      (Game|Player|SetViewTargetwithBlend (Game|GetPlayerController (LocalVariables|GetIndex)) (Variables|References|GetCameraRef) 0.0 "VTBlend_Linear" 0.0 false)
      (else
        (Input|AddMappingContext (PlayerController|LocalPlayerSubsystems|GetEnhancedInputLocalPlayerSubsystem (Game|GetPlayerController 0)) "/Game/GameMode2/Design/Input/IMC_GM2_Default.IMC_GM2_Default" 0 "(bIgnoreAllPressedKeysUntilRelease=True,bForceImmediately=False)")
        (bind _returnvalue_4 (Game|SpawnActorfromClass "/Game/GameMode2/Programming/Gamemode/BP_GM2_InputReciever.BP_GM2_InputReciever_C" (Transformation|GetActorTransform (Utilities|Array|Get(acopy) (Variables|PlayerData|GetPlayerStarts) (LocalVariables|GetIndex))) "Undefined" "MultiplyWithRoot" 0 (LocalVariables|GetIndex) 0))
        (Utilities|Array|AddUnique (Variables|PlayerData|GetPlayerInputRecievers) _returnvalue_4)
        (Pawn|Possess _returnvalue _returnvalue_4)
        (Utilities|Array|AddUnique (Variables|PlayerData|GetPlayerControllers) _returnvalue)
        (Game|Player|SetViewTargetwithBlend (Game|GetPlayerController 0) (Variables|References|GetCameraRef) 0.0 "VTBlend_Linear" 0.0 false)))))

(fn GameStarted
  (Variables|Default|SetisInGame true)
  (CallFunction|BeginTimeLimitObjective)
  (Development|PrintString "Game Started")
  (Default|IncrementNumGamesPlayed (Variables|References|GetGame%20Instance)))

(fn RemoveUnusedCameras)

(fn CacheGlobals
  ;[1 1 1] Camera
  (bind _outactors (Actor|GetAllActorsOfClass "/Script/Engine.CameraActor"))
  (Variables|References|SetCameraRef (Utilities|Array|Get(acopy) _outactors))
  ;[1 1 1] Player Starts
  (bind _outactors_2 (Actor|GetAllActorsOfClass "/Script/Engine.PlayerStart"))
  (Variables|PlayerData|SetPlayerStarts _outactors_2)
  ;[1 1 1] Game Instance
  (bind _asgi_core_game_instance (Utilities|Casting|CastToGI_CORE_GameInstance (Game|GetGameInstance))
    (:then
      (bind _output_get (Variables|References|SetGame%20Instance _asgi_core_game_instance))
      (bind _valid (Default|HasPlayers _output_get))
      (if _valid
        _
        (else
          (Development|PrintString "GM_GM2 :: Game instance has no players. Make sure you play this level through the lobby to enable multiplayer. For editor purposes, this will start the level in single player. 
 
The lobby level is at /Content/Core/Programming/Prototypes/Lobby/Lobby" true true "(R=0.000000,G=0.660000,B=1.000000,A=1.000000)" 1e+01)))
      (return (not _valid)))
    (:CastFailed
      (Development|PrintString "GM_GM2 :: Game instance is the wrong type.")
      (return true))))

(fn SpawnPlayersfromGameInstance
  (bind _game_instance (Variables|References|GetGame%20Instance))
  (for (_ _array_index) (Variables|/Game/Core/Programming/Prototypes/GameData/GI_CORE_GameInstance.GI_CORE_GameInstance_C|GetPlayerData _game_instance)
    (bind _connected (Default|GetPlayerConnected _game_instance _array_index))
    (if _connected
      (CallFunction|SpawnPlayer (Utilities|Array|Get(acopy) (Variables|PlayerData|GetPlayerStarts) _array_index) _array_index))))

(fn GetWinner
  (bind _players (Variables|PlayerData|GetPlayers))
  (LocalVariables|SetWinning%20Player (Utilities|Array|Get(acopy) _players))
  (for _array_element _players
    ;[1 1 1] Find the winner
    (bind _score (Default|GetScore _array_element))
    (bind _score_2 (Default|GetScore (LocalVariables|GetWinning%20Player)))
    (if (> _score_2 _score)
      (LocalVariables|SetWinning%20Player _array_element)))
  (return (LocalVariables|GetWinning%20Player)))

(fn ShowWinner
  (bind _player (CallFunction|GetWinner))
  ;[1 1 1] WINNNN
  (bind _returnvalue (UserInterface|CreateWidget "/Game/GameMode2/Programming/UI/WBP_GM2_Win.WBP_GM2_Win_C" (Pawn|GetLocalViewingPlayerController _player)))
  (UserInterface|Viewport|AddtoViewport _returnvalue 0)
  (Default|ShowWinner _returnvalue (Variables|PlayerData|GetPlayers) _player))

(fn InitializeHUD
  (bind _returnvalue (Game|GetPlayerController 0))
  (bind _returnvalue_2 (HUD|GetHUD _returnvalue))
  (bind _ashud_gm2 (Utilities|Casting|CastToHUD_GM2 _returnvalue_2))
  (Default|Initialize _ashud_gm2)
  ;[0.1317 0.5622 1] Potential fix for HUD not showing if no player 0
  (for _array_element (Variables|PlayerData|GetPlayers)
    (bind _connected (Default|GetPlayerConnected (Variables|References|GetGame%20Instance) (Variables|/Game/GameMode2/Programming/Movement/PC_GM2_Player.PC_GM2_Player_C|GetPlayer%20Number _array_element)))
    (if _connected
      (Default|AddPlayer _ashud_gm2 _array_element (Variables|/Game/GameMode2/Programming/Movement/PC_GM2_Player.PC_GM2_Player_C|GetPlayer%20Number _array_element))
      (else
        (Development|PrintText (Utilities|Text|FormatText "FALSE Before Add Player; Index: {0}" (Variables|/Game/GameMode2/Programming/Movement/PC_GM2_Player.PC_GM2_Player_C|GetPlayer%20Number _array_element)))))))

(fn GotoNextLevel
  (Game|OpenLevel(byObjectReference) "/Game/Core/Programming/Prototypes/Test_Kellyn/Maps/MidGameResultsScreen.MidGameResultsScreen"))

(fn SavePlayerScores
  (bind _game_instance (Variables|References|GetGame%20Instance))
  (for _array_element (Variables|PlayerData|GetPlayers)
    (bind _score (Default|GetScore _array_element))
    (Default|AddPlayerScore _game_instance _score (Variables|/Game/GameMode2/Programming/Movement/PC_GM2_Player.PC_GM2_Player_C|GetPlayer%20Number _array_element))
    (Default|AddWins _game_instance)))

(fn Announce
  (Default|CallOnEndGame)
  (Development|PrintString "[ANNOUNCE WINNER]" true true "(R=1.000000,G=0.747086,B=0.100902,A=1.000000)" 5e+01)
  (Default|CallGM2GameEnd (Variables|Default|GetFXManager))
  (Utilities|Time|SetTimerbyFunctionName 0 "GoToNextLevel" 3.0))

(fn GetIsinGame
  (return (Variables|Default|GetisInGame)))

(fn SpawnPlayer
  (params (Player%20Start :type Player%20Start%20Object%20Reference) (Game%20Instance%20ID :type Integer))
  (bind _returnvalue (Transformation|GetActorTransform Player%20Start))
  (bind _returnvalue_2 (Game|GetPlayerController Game%20Instance%20ID))
  (bind _da_gm2_player (Variables|References|GetDA_GM2_Player))
  (bind _ballsize (Variables|/Game/GameMode2/Programming/PLAYERDATA/DA_Player.DA_Player_C|GetBallSize _da_gm2_player))
  ;[0 0 0 0.5] Spawn Player Pawn and Possess
  (bind _returnvalue_3 (Game|SpawnActorfromClass "/Game/GameMode2/Programming/Movement/PC_GM2_Player.PC_GM2_Player_C" _returnvalue "Undefined" "MultiplyWithRoot" 0 (Variables|/Game/GameMode2/Programming/Gamemode/DA_GM2_Objective.DA_GM2_Objective_C|GetPregame%20Countdown%20Length (Variables|References|GetObjective)) Game%20Instance%20ID 1 0))
  (Utilities|Array|Add (Variables|PlayerData|GetPlayers) _returnvalue_3)
  (Default|Initialize _returnvalue_3 Game%20Instance%20ID _returnvalue)
  (Pawn|Possess _returnvalue_2 _returnvalue_3)
  (Game|Player|SetViewTargetwithBlend _returnvalue_2 (Variables|References|GetCameraRef) 0.0 "VTBlend_Linear" 0.0 false)
  ;[0.5276 1 0.1747] Set Player Scale on spawn to match BallSize in DA_GM2_Player (Sai)
  (for _array_element (Variables|PlayerData|GetPlayers)
    (Utilities|IsValid _da_gm2_player
      (:Is%20Valid
        (Transformation|SetActorRelativeScale3D _array_element (Math|Vector|MakeVector _ballsize _ballsize _ballsize)))))
  (return))

(fn StartGame
  (CallFunction|GameStarted)
  (Default|CallOnStartGame)
  (Default|CallGM2GameStart (Variables|Default|GetFXManager))
  (Default|CallPlatforms)
  (return false))