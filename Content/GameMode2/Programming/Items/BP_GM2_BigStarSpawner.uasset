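; Big star spawner for GameMode2 that refills BP_GM2_BigStarSpawnPoint actors cached at BeginPlay.
; After an initial delay it attempts batches of spawns on points without a collectible or nearby player, then waits a random DAPlayer delay, polling first while none are free.
; ForceBigSpawnStar requests an immediate spawn.
; GetRandomSpawner only returns a point when exactly one is eligible, with no random pick among several.
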(event Custom|Setup
  (Utilities|Casting|CastToPC_GM2_Player (Game|Player|GetPlayerPawn 0)))

(event Custom|ForceBigSpawnStar
  (bind _spawners (CallFunction|GetEmptySpawners))
  (if (!= (Utilities|Array|Length _spawners) 0)
    (bind _spawner (CallFunction|GetRandomSpawner _spawners))
    (Default|SpawnCollectible _spawner)
    (Development|PrintString "Lost Star Spawned")))

(event EventBeginPlay
  (bind _da_player (Variables|Default|GetDA_Player))
  (bind _delayrangeforbigstar (Variables|/Game/GameMode2/Programming/PLAYERDATA/DA_Player.DA_Player_C|GetDelayRangeForBigStar _da_player))
  (CallFunction|Setup)
  ;[1 1 1] Cache Spawners
  (bind _outactors (Actor|GetAllActorsOfClass "/Game/GameMode2/Design/Powerups/BP_GM2_BigStarSpawnPoint.BP_GM2_BigStarSpawnPoint_C"))
  (Variables|Default|SetSpawn%20Points _outactors)
  (Utilities|FlowControl|Delay (Variables|/Game/GameMode2/Programming/PLAYERDATA/DA_Player.DA_Player_C|GetInitialBigStarDelay (Variables|Default|GetDA_Player)))
  (bind _output_get (Variables|Default|Set_Counter 0 :!label _label))
  (while (< _output_get (Variables|Default|GetSpawn%20Amount))
    ;[1 1 1] Randomly Refill Collectible Slots
    (Math|Integer|IncrementInt (Variables|Default|Get_Counter)
      (:%20%20
        (bind _spawners (CallFunction|GetEmptySpawners))
        (if (!= 0 (Utilities|Array|Length _spawners))
          (bind _spawner (CallFunction|GetRandomSpawner _spawners))
          (Utilities|IsValid _spawner
            (:Is%20Valid
              (Default|SpawnCollectible _spawner)))))))
  (bind _spawners_2 (CallFunction|GetEmptySpawners :!label _label_2))
  ;[1 1 1] Don't do random delay till a collector is empty
  (if (> (Utilities|Array|Length _spawners_2) 0)
    ;[1 1 1] Randomly wait for next spawn
    (Utilities|FlowControl|Delay (Utilities|RandomFloatinRange (Game|GetGameInstance) (.x _delayrangeforbigstar) (.y _delayrangeforbigstar)))
    (goto _label)
    (else
      (Utilities|FlowControl|Delay 0.1)
      (goto _label_2))))

(fn ConstructionScript)

(fn GetEmptySpawners
  (LocalVariables|Setresult (Utilities|Array|MakeArray))
  (for _array_element (Variables|Default|GetSpawn%20Points)
    (bind _value (Default|HasCollectible _array_element))
    (bind _player_is_near (Default|HasPlayerNearby _array_element))
    (if (not (or _player_is_near _value))
      (Utilities|Array|Add (LocalVariables|Getresult) _array_element)))
  (return (LocalVariables|Getresult)))

(fn GetRandomSpawner
  (params (Spawners :type Array%20of%20BP%20GM2%20Big%20Star%20Spawn%20Point%20Object%20References))
  (bind _returnvalue (Utilities|Array|Length Spawners))
  ;[1 1 1] Skip trival cases
  (if (== _returnvalue 0)
    (return 0)
    (elif (== _returnvalue 1)
      (return (Utilities|Array|Get(acopy) Spawners)))))

(fn AllSpawnersFull
  (for _array_element (Variables|Default|GetSpawn%20Points)
    (bind _value (Default|HasCollectible _array_element))
    (bind _player_is_near (Default|HasPlayerNearby _array_element))
    (if (not (or _player_is_near _value))
      (return false)))
  (return true))

(fn AllSpawnersEmpty
  (for _array_element (Variables|Default|GetSpawn%20Points)
    (bind _value (Default|HasCollectible _array_element))
    (bind _player_is_near (Default|HasPlayerNearby _array_element))
    (if (or _player_is_near _value)
      (return false)))
  (return true))