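; Big star powerup for GameMode2 that awards data-asset-defined points to the player who collects it.
; On spawn it randomly varies its rotation speed and takes color and scale from DAPlayer, using a dynamic material instance.
; Spawn and collection are reported to the game mode's FX manager.
; The construction script binds spawn and collect events, but their visible handlers are empty and the sound calls are unwired.
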(event Custom|OnLargeStarCollectedEvent)

(event Custom|OnLargeStarSpawnEvent
  (params (Location :type Vector)))

(event Custom|BigStarCollectTest_Event)

(event EventBeginPlay
  (bind _rotatingmovement (Variables|Default|GetRotatingMovement))
  (bind _da_player (Variables|Default|GetDA_Player))
  (bind _asgm_gm2 (Utilities|Casting|CastToGM_GM2 (Game|GetGameMode)))
  (Variables|Default|SetFXEventManager (Variables|/Game/GameMode2/Programming/Gamemode/GM_GM2.GM_GM2_C|GetFXManager _asgm_gm2))
  (Default|CallOnLargeStarSpawn (Transformation|GetActorLocation))
  (Default|CallGM2LargeStarSpawn (Variables|Default|GetFXEventManager) self)
  (Variables|/Script/Engine.RotatingMovementComponent|SetRotationRate _rotatingmovement (Math|Rotator|CombineRotators (Variables|/Script/Engine.RotatingMovementComponent|GetRotationRate _rotatingmovement) (* (Variables|/Script/Engine.RotatingMovementComponent|GetRotationRate _rotatingmovement) (Utilities|RandomFloatinRange (Game|GetGameInstance) -0.25 0.25))))
  (bind _returnvalue (Rendering|Material|CreateDynamicMaterialInstance (Variables|Default|GetSM_Star) 0 "/Game/GameMode2/Art/Powerups/Star/Source/M_Star.M_Star" "None" :!class /Script/Engine.PrimitiveComponent))
  (Rendering|Material|SetVectorParameterValue _returnvalue "Color" (Variables|/Game/GameMode2/Programming/PLAYERDATA/DA_Player.DA_Player_C|GetBigStarColor _da_player) :!class /Script/Engine.MaterialInstanceDynamic)
  (Transformation|SetRelativeScale3D (Variables|Default|GetDefaultSceneRoot) (Variables|/Game/GameMode2/Programming/PLAYERDATA/DA_Player.DA_Player_C|GetBigStarSize _da_player)))

(fn ConstructionScript
  (|CallParentFunction)
  (EventDispatchers|BindEventtoOnLargeStarCollected (EventDispatchers|CreateEvent :!event Custom|OnLargeStarCollectedEvent))
  (EventDispatchers|BindEventtoOnLargeStarSpawn (EventDispatchers|CreateEvent :!event Custom|OnLargeStarSpawnEvent)))

(fn Collected
  (params (Player :type PC%20GM2%20Player%20Object%20Reference))
  (|CallParentFunction Player)
  (Default|AddtoScore Player (Variables|/Game/GameMode2/Programming/PLAYERDATA/DA_Player.DA_Player_C|GetBigStarPoints (Variables|Default|GetDA_Player)))
  (Default|CallGM2LargeStarCollected (Variables|Default|GetFXEventManager) self)
  (Development|PrintString "Super Star End"))