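; Star powerup for game mode GM2 that adds its points to the collecting player's score and broadcasts a collected event.
; On BeginPlay it registers with the game mode's FX manager, broadcasts its spawn event and randomly varies its rotation speed by up to 25% either way.
; The local spawn VFX and the binding to the spawn dispatcher are disconnected, leaving the spawn sound event unbound within this Blueprint.
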(event Custom|OnStarSpawnEvent
  ;[1 1 1] OnStarSpawn
  (Audio|PlaySoundatLocation (Variables|Default|GetSFX_Spawned) (Transformation|GetActorLocation) "0, 0, 0" 1.0 1.0 0.0 0 0 0 0))

(event EventBeginPlay
  (bind _rotatingmovement (Variables|Default|GetRotatingMovement))
  (bind _asgm_gm2 (Utilities|Casting|CastToGM_GM2 (Game|GetGameMode)))
  (Variables|Default|SetFXEventManager (Variables|/Game/GameMode2/Programming/Gamemode/GM_GM2.GM_GM2_C|GetFXManager _asgm_gm2))
  (Default|CallGM2StarSpawn (Variables|Default|GetFXEventManager) self)
  (Default|CallOnStarSpawn)
  (Variables|/Script/Engine.RotatingMovementComponent|SetRotationRate _rotatingmovement (Math|Rotator|CombineRotators (Variables|/Script/Engine.RotatingMovementComponent|GetRotationRate _rotatingmovement) (* (Variables|/Script/Engine.RotatingMovementComponent|GetRotationRate _rotatingmovement) (Math|Random|RandomFloatinRange -0.25 0.25)))))

(fn ConstructionScript
  (|CallParentFunction))

(fn Collected
  (params (Player :type PC%20GM2%20Player%20Object%20Reference))
  (|CallParentFunction Player)
  (Default|AddtoScore Player (Variables|Default|GetPoints))
  (Default|CallOnStarCollected))