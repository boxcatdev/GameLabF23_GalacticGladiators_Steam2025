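; Spawn point for GameMode2 collectibles that spawns an instance of its configured type on demand, guarded against duplicate spawns.
; A pre-spawn event and VFX precede a delay, then the collectible spawns attached to the point alongside idle VFX.
; Destruction of the collectible clears the idle VFX and timestamps TimeOfLastSelection.
; An overlap volume counts nearby players, exposed through HasPlayerNearby alongside HasCollectible.
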(event OnComponentEndOverlap(PlayerDetectorCollision)
  (params (OverlappedComponent :type Primitive%20Component%20Object%20Reference) (OtherActor :type Actor%20Object%20Reference) (OtherComp :type Primitive%20Component%20Object%20Reference) (OtherBodyIndex :type Integer))
  (Utilities|Casting|CastToPC_GM2_Player OtherActor)
  (Variables|Default|SetPlayers%20Nearby (- (Variables|Default|GetPlayers%20Nearby) 1)))

(event OnComponentBeginOverlap(PlayerDetectorCollision)
  (params (OverlappedComponent :type Primitive%20Component%20Object%20Reference) (OtherActor :type Actor%20Object%20Reference) (OtherComp :type Primitive%20Component%20Object%20Reference) (OtherBodyIndex :type Integer) (bFromSweep :type Boolean) (SweepResult :type Hit%20Result%20Structure%20%28by%20ref%29))
  (Utilities|Casting|CastToPC_GM2_Player OtherActor)
  (Variables|Default|SetPlayers%20Nearby (+ (Variables|Default|GetPlayers%20Nearby) 1)))

(event Custom|Spawn%20Collectible
  (bind _returnvalue (Transformation|GetActorTransform))
  (bind _returnvalue_2 (Transformation|GetActorTransform))
  (bind (_location _rotation _scale) (Math|Transform|BreakTransform _returnvalue))
  (bind (_location_2 _rotation_2 _scale_2) (Math|Transform|BreakTransform _returnvalue_2))
  (bind (_location_3 _rotation_3 _scale_3) (Math|Transform|BreakTransform _returnvalue_2))
  ;[1 1 1] Stop Multiple Spawns
  (bind _value (CallFunction|HasCollectible))
  (if (not _value)
    (Variables|Default|SetIs%20about%20to%20spawn true)
    (Default|CallOnStarPreSpawn)
    ;[1 1 1] Prespawn VFX
    (bind _returnvalue_3 (Niagara|SpawnSystematLocation (Variables|Default|GetPrespawn%20VFX) _location_3 _rotation_3 _scale_3))
    (Variables|Default|SetIdle%20VFX%20Instance _returnvalue_3)
    ;[1 1 1] Wait for prespawn phase to end
    (Utilities|FlowControl|Delay (Variables|Default|GetDelay%20between%20vfx%20and%20spawn))
    (Variables|Default|SetIs%20about%20to%20spawn false)
    ;[1 1 1] Spawn Collectible
    (bind _returnvalue_4 (Game|SpawnActorfromClass (Variables|Default|GetSpawned%20Type) (Math|Transform|MakeTransform (+ _location_2 (Math|Vector|MakeVector 0.0 0.0 (Variables|Default|GetSpawned%20Vertical%20Offset))) _rotation_2 _scale_2) "Undefined" "MultiplyWithRoot" 0 0))
    (bind _output_get (Variables|Default|SetCollectible%20Instance _returnvalue_4))
    (Utilities|IsValid _output_get
      (:Is%20Valid
        (Transformation|AttachComponentToComponent _returnvalue_4 (Variables|Default|GetDefaultSceneRoot) "None" "SnapToTarget" "KeepRelative" "KeepRelative" true)
        ;[1 1 1] Idle VFX
        (bind _returnvalue_5 (Niagara|SpawnSystematLocation (Variables|Default|GetIdle%20VFX) _location _rotation _scale false))
        (Variables|Default|SetIdle%20VFX%20Instance _returnvalue_5)
        (Utilities|IsValid _output_get
          (:Is%20Valid
            (Game|BindEventtoOnDestroyed _output_get (delegate Custom|Destroy%20Idle%20VFX)))))
      (:Is%20Not%20Valid
        ;[1 1 1] Remove VFX on collection
        (bind _idle_vfx_instance (Variables|Default|GetIdle%20VFX%20Instance)
          (:then
            (Components|DestroyComponent _idle_vfx_instance)
            (Variables|Default|SetTime%20of%20last%20selection (Utilities|Time|GetGameTimeinSeconds)))
          (:else))))))

(event Custom|Destroy%20Idle%20VFX
  (params (DestroyedActor :type Actor%20Object%20Reference))
  ;[1 1 1] Remove VFX on collection
  (bind _idle_vfx_instance (Variables|Default|GetIdle%20VFX%20Instance)
    (:then
      (Components|DestroyComponent _idle_vfx_instance)
      (Variables|Default|SetTime%20of%20last%20selection (Utilities|Time|GetGameTimeinSeconds)))
    (:else)))

(fn ConstructionScript)

(fn HasCollectible
  (return (or (Variables|Default|GetIs%20about%20to%20spawn) (Utilities|IsValid (Variables|Default|GetCollectible%20Instance)))))

(fn HasPlayerNearby
  (return (> (Variables|Default|GetPlayers%20Nearby) 0)))