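; BP_Bumper is a GM1 hazard that rises through animated hatches after a brief decal warning and launches players who hit it.
; Hits bounce the player horizontally along their reflected velocity, with animation, sound and FXManager effects.
; A timeline lerps the bumper's height when raising and reverses to lower it.
; Editor-only functions save or append bumper locations to a stage hazard data asset; another respawns bumpers from it.
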(event Custom|RaiseBumper
  (bind _bumper (Variables|Default|GetBumper))
  (bind _returnvalue (Transformation|GetWorldLocation _bumper))
  ;[0 0 0] Briefly display warning
  (Development|SetHiddeninGame (Variables|Default|GetDecalWarning) false false)
  (Utilities|FlowControl|Delay 3.0)
  (Development|SetHiddeninGame (Variables|Default|GetDecalWarning) true false)
  (bind _asgm_gm1 (Utilities|Casting|CastToGM_GM1 (Game|GetGameMode)))
  (Default|CallGM1HazardBumpersRaise (Variables|/Game/Systems/Blueprints/GM1/Systems/GM_GM1.GM_GM1_C|GetFXManager _asgm_gm1) self)
  (Components|Animation|PlayAnimation (Variables|Default|GetBumperHatches) "/Game/GameMode1/Art/Stage_Animations/Bumper_Animations/SK_BumperHatch_Open_Anim.SK_BumperHatch_Open_Anim" false)
  (Utilities|FlowControl|Delay 1.0)
  ;[0 0 0] Animate bumper towards target
  (bind _alpha (Timeline|Rise Play)
    (:Update
      (Transformation|SetWorldLocation _bumper (Math|Vector|MakeVector (.x _returnvalue) (.y _returnvalue) (Math|Float|Lerp (.z _returnvalue) 25.0 _alpha)) false false))
    (:Finished
      (Components|Animation|PlayAnimation (Variables|Default|GetBumperHatches) "/Game/GameMode1/Art/Stage_Animations/Bumper_Animations/SK_BumperHatch_Close_Anim.SK_BumperHatch_Close_Anim" false))))

(event Custom|LowerBumper
  (bind _bumper (Variables|Default|GetBumper))
  (bind _returnvalue (Transformation|GetWorldLocation _bumper))
  (bind _asgm_gm1 (Utilities|Casting|CastToGM_GM1 (Game|GetGameMode)))
  (Default|CallGM1HazardBumpersLower (Variables|/Game/Systems/Blueprints/GM1/Systems/GM_GM1.GM_GM1_C|GetFXManager _asgm_gm1) self)
  ;[0 0 0] Animate bumper towards target
  (bind _alpha (Timeline|Rise Reverse)
    (:Update
      (Transformation|SetWorldLocation _bumper (Math|Vector|MakeVector (.x _returnvalue) (.y _returnvalue) (Math|Float|Lerp (.z _returnvalue) 25.0 _alpha)) false false))
    (:Finished
      (Components|Animation|PlayAnimation (Variables|Default|GetBumperHatches) "/Game/GameMode1/Art/Stage_Animations/Bumper_Animations/SK_BumperHatch_Close_Anim.SK_BumperHatch_Close_Anim" false))))

(event EventBeginPlay
  (Variables|Default|SetbaseZ (.Z (Class|KismetMathLibrary|BreakVector3f (Transformation|GetActorLocation))))
  (Components|Animation|PlayAnimation (Variables|Default|GetBumper) "/Game/GameMode1/Art/Stage_Animations/Bumper_Animations/BumperAnim_Armature_Idle.BumperAnim_Armature_Idle" false))

(event Collision|EventHit
  (params (MyComp :type Primitive%20Component%20Object%20Reference) (Other :type Actor%20Object%20Reference) (OtherComp :type Primitive%20Component%20Object%20Reference) (bSelfMoved :type Boolean) (HitLocation :type Vector :default "0, 0, 0") (HitNormal :type Vector :default "0, 0, 0") (NormalImpulse :type Vector :default "0, 0, 0") (Hit :type Hit%20Result%20Structure%20%28by%20ref%29))
  ;[0 0 0] If we hit a player, bounce that player and play animation
  (bind _asbp_player_gm1 (Utilities|Casting|CastToBP_Player_GM1 Other))
  (CallFunction|Bump _asbp_player_gm1 (Math|Vector|GetReflectionVector (Transformation|GetVelocity Other) (* HitNormal -1.0))) ; Bump seems to trigger twice on every hit, but it doesn't seem to cause any issues yet. This is less expensive, so it's better for now
  (Components|Animation|PlayAnimation (Variables|Default|GetBumper) "/Game/GameMode1/Art/Stage_Animations/Bumper_Animations/BumperAnim1_Bump.BumperAnim1_Bump" false))

(fn ConstructionScript)

(fn Bump
  (params (player :type BP%20Player%20GM1%20Object%20Reference) (direction :type Vector))
  (bind _returnvalue (Math|Vector|Normalize direction))
  (bind _bouncevelocity (Variables|Default|GetbounceVelocity))
  (bind _returnvalue_2 (* _returnvalue _bouncevelocity))
  (bind (_x _y) (Math|Vector|BreakVector _returnvalue_2))
  ;[0 0 0] Boink the player
  (Character|LaunchCharacter player (Math|Vector|MakeVector _x _y 0.0) true false)
  (Audio|PlaySound2D 0 1.0 1.0 0.0 0 0)
  (bind _asgm_gm1 (Utilities|Casting|CastToGM_GM1 (Game|GetGameMode)))
  (Default|CallGM1HazardBumpersCollision (Variables|/Game/Systems/Blueprints/GM1/Systems/GM_GM1.GM_GM1_C|GetFXManager _asgm_gm1) self player))

(fn SaveBumperLocations
  ;[0 0 0] EDITOR ONLY: Save the location of all bumpers in current level to the bumper hazard data asset, overwriting any previously saved data, then destroy those bumpers
  (bind _outactors (Actor|GetAllActorsOfClass "BP_Bumper_C"))
  (if (!= (Utilities|Array|Length _outactors) 0)
    (Default|CopyLocationsOfBumpers (Variables|Default|GetStageHazardData) _outactors)
    (for _array_element _outactors
      (Actor|DestroyActor _array_element))))

(fn AddBumperLocations
  ;[0 0 0] EDITOR ONLY: Save the location of all bumpers in current level to the bumper hazard data asset, appending to any previously saved data, then destroy those bumpers
  (bind _outactors (Actor|GetAllActorsOfClass "BP_Bumper_C"))
  (if (!= (Utilities|Array|Length _outactors) 0)
    (Default|AddLocationsOfBumpers (Variables|Default|GetStageHazardData) _outactors)
    (for _array_element _outactors
      (Actor|DestroyActor _array_element))))

(fn SpawnSavedBumpers
  ;[0 0 0] Destroy any bumpers in the level
  (bind _outactors (Actor|GetAllActorsOfClass "BP_Bumper_C"))
  (for _array_element _outactors
    (Actor|DestroyActor _array_element))
  ;[0 0 0] Spawn a bumper at each location saved to the bumper hazard data asset
  (for _array_element_2 (Variables|/Game/Systems/Blueprints/GM1/Hazards/Data/PDA_BumperHazard.PDA_BumperHazard_C|GetBumperLocations (Variables|Default|GetStageHazardData))
    (Game|SpawnActorfromClass "BP_Bumper_C" (Math|Conversions|ToTransform(Vector) _array_element_2) "AlwaysSpawn" "MultiplyWithRoot" 0 0 0)))