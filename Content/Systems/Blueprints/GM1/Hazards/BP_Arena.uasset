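; GM1 arena hazard actor with two hazards: a spreading ice ring and a player-driven tilting floor.
; Ice flashes a warning material, then a timeline shrinks the ground collision alongside a dynamic decal's inner ring, with GM_GM1's FXManager notified.
; While tilting, Tick sums overlapping players' offsets, clamped to arena radius, into a smoothed target rotation with eased tilt speed for momentum.
; Stopping tilt eases rotation back to level.
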(event Custom|StartTilt
  (Variables|Tilt|SetIsTilting true)
  (Development|PrintString "Tilt Hazard Started" true true "(R=0.000000,G=0.710069,B=0.055656,A=1.000000)"))

(event Custom|StopTilt
  (Variables|Tilt|SetIsTilting false)
  (Development|PrintString "Tilt Hazard Stopped" true true "(R=1.000000,G=0.187080,B=0.000000,A=1.000000)")
  (bind _alpha (Timeline|ReturnToBaseRotation PlayFromStart)
    (:Update
      (Transformation|SetActorRotation (Math|Interpolation|RInterpTo (Transformation|GetActorRotation) "0, 0, 0" (Utilities|Time|GetWorldDeltaSeconds) _alpha)))))

(event Custom|Start%20Ice%20Grow
  (bind _asgm_gm1 (Utilities|Casting|CastToGM_GM1 (Game|GetGameMode)))
  (Default|CallGM1HazardIceSpreading (Variables|/Game/Systems/Blueprints/GM1/Systems/GM_GM1.GM_GM1_C|GetFXManager _asgm_gm1) true)
  ;[0 0 0] Display a brief warning
  (Rendering|Material|SetMaterial (Variables|Default|GetGroundCollision) 0 "/Game/GameMode1/Art/Materials/MI_OverlayGlow.MI_OverlayGlow")
  (Utilities|FlowControl|Delay 3.0)
  (Rendering|Material|SetMaterial (Variables|Default|GetGroundCollision) 0 "/Game/GameMode1/Art/LevelPrototyping/MI_Whitebox.MI_Whitebox")
  (Rendering|SetVisibility (Variables|Default|GetIceVisuals) true false)
  (bind _returnvalue (Rendering|Material|CreateDynamicMaterialInstance "/Game/GameMode1/Art/Decals/GM1/MI_GM1_SurfaceDecal_IceRing.MI_GM1_SurfaceDecal_IceRing" "None" "None" :!class /Script/Engine.KismetMaterialLibrary))
  (Rendering|Components|Decal|SetDecalMaterial (Variables|Default|GetIceVisuals) _returnvalue)
  (Variables|Default|SetIceRingMaterial _returnvalue)
  (bind _alpha (Timeline|Timeline Play)
    (:Update
      ;[0 0 0] Animate the ice ground collision's size towards the minimum
      (Transformation|SetRelativeScale3D (Variables|Default|GetGround) (Math|Vector|MakeVector (Math|Float|Lerp 1.0 (Variables|/Game/Systems/Blueprints/GM1/Hazards/Data/PDA_IceHazard.PDA_IceHazard_C|GetEndScale (Variables|Default|GetIceRingData)) _alpha) (Math|Float|Lerp 1.0 (Variables|/Game/Systems/Blueprints/GM1/Hazards/Data/PDA_IceHazard.PDA_IceHazard_C|GetEndScale (Variables|Default|GetIceRingData)) _alpha) (.Z (Math|Vector|BreakVector (Variables|/Script/Engine.SceneComponent|GetRelativeScale3D (Variables|Default|GetGround))))))
      ;[0 0 0] Animate the ice ring decal's size towards the minimum
      (Rendering|Material|SetScalarParameterValue (Variables|Default|GetIceRingMaterial) "InnerRingSize" (Math|Float|Lerp 1.0 (Variables|/Game/Systems/Blueprints/GM1/Hazards/Data/PDA_IceHazard.PDA_IceHazard_C|GetEndScale (Variables|Default|GetIceRingData)) _alpha) :!class /Script/Engine.MaterialInstanceDynamic))))

(event Custom|Stop%20Ice%20Grow
  (bind _asgm_gm1 (Utilities|Casting|CastToGM_GM1 (Game|GetGameMode)))
  (Default|CallGM1HazardIceSpreading (Variables|/Game/Systems/Blueprints/GM1/Systems/GM_GM1.GM_GM1_C|GetFXManager _asgm_gm1) false)
  (bind _alpha (Timeline|Timeline Stop)
    (:Update
      ;[0 0 0] Animate the ice ground collision's size towards the minimum
      (Transformation|SetRelativeScale3D (Variables|Default|GetGround) (Math|Vector|MakeVector (Math|Float|Lerp 1.0 (Variables|/Game/Systems/Blueprints/GM1/Hazards/Data/PDA_IceHazard.PDA_IceHazard_C|GetEndScale (Variables|Default|GetIceRingData)) _alpha) (Math|Float|Lerp 1.0 (Variables|/Game/Systems/Blueprints/GM1/Hazards/Data/PDA_IceHazard.PDA_IceHazard_C|GetEndScale (Variables|Default|GetIceRingData)) _alpha) (.Z (Math|Vector|BreakVector (Variables|/Script/Engine.SceneComponent|GetRelativeScale3D (Variables|Default|GetGround))))))
      ;[0 0 0] Animate the ice ring decal's size towards the minimum
      (Rendering|Material|SetScalarParameterValue (Variables|Default|GetIceRingMaterial) "InnerRingSize" (Math|Float|Lerp 1.0 (Variables|/Game/Systems/Blueprints/GM1/Hazards/Data/PDA_IceHazard.PDA_IceHazard_C|GetEndScale (Variables|Default|GetIceRingData)) _alpha) :!class /Script/Engine.MaterialInstanceDynamic))))

(event EventTick
  (params (DeltaSeconds :type Float%20%28single-precision%29))
  (if (Variables|Tilt|GetIsTilting)
    (CallFunction|DynamicTilt)))

(event EventBeginPlay
  (bind _iceringmaterial (Variables|Default|GetIceRingMaterial))
  (Components|DestroyComponent (Variables|Default|GetIndicator))
  (Rendering|SetVisibility (Variables|Default|GetIceVisuals) false false)
  (Utilities|IsValid _iceringmaterial
    (:Is%20Valid
      (Rendering|Material|SetScalarParameterValue _iceringmaterial "InnerRingSize" 1.0 :!class /Script/Engine.MaterialInstanceDynamic))))

(fn ConstructionScript)

(fn DynamicTilt
  (bind _x (Utilities|RadiusinUnits))
  (bind _scale (Utilities|ScaleinUnits))
  (bind _arenatiltdata (Variables|Tilt|GetArenaTiltData))
  (bind _arenatiltdata_2 (Variables|Tilt|GetArenaTiltData))
  (bind (_x_2 _y) (Math|Vector|BreakVector _scale))
  (bind _maxtilt (Variables|/Game/Systems/Blueprints/GM1/Hazards/Data/PDA_ArenaTilt.PDA_ArenaTilt_C|GetMaxTilt _arenatiltdata))
  (bind (_x_3 _y_2) (Math|Vector|BreakVector _maxtilt))
  ;[0 0 0 0.25] Rotate arena towards target rotation
  (LocalVariables|Setplayers (Collision|GetOverlappingActors (Variables|Default|GetPlayerCheck) "/Game/Systems/Blueprints/GM1/Player/Blueprints/BP_Player_GM1.BP_Player_GM1_C" :!class /Script/Engine.PrimitiveComponent))
  (Variables|Tilt|SetcurrentTiltSpeed (Math|Interpolation|FInterpTo (Variables|Tilt|GetcurrentTiltSpeed) (Math|Float|SelectFloat 0.0 (Variables|/Game/Systems/Blueprints/GM1/Hazards/Data/PDA_ArenaTilt.PDA_ArenaTilt_C|GetmaxTiltSpeed _arenatiltdata_2) (Utilities|Operators|EqualEqual (Variables|Tilt|GetTargetRotation) (Transformation|GetActorRotation) 0.05)) (Utilities|Time|GetWorldDeltaSeconds) (Variables|/Game/Systems/Blueprints/GM1/Hazards/Data/PDA_ArenaTilt.PDA_ArenaTilt_C|GetTiltAcceleration _arenatiltdata_2)))
  (Transformation|SetActorRotation (Class|KismetMathLibrary|RInterptoConstant (Transformation|GetActorRotation) (Variables|Tilt|GetTargetRotation) (Utilities|Time|GetWorldDeltaSeconds) (Variables|Tilt|GetcurrentTiltSpeed)))
  ;[0 0 0 0.25] Calculate new target rotation based on player positions
  ;;[0 0 0] Get the net distance of players from the center of the arena
  (Utilities|Array|Clear (LocalVariables|GetplayerDistances))
  (for _array_element (LocalVariables|Getplayers)
    (Utilities|Array|Add (LocalVariables|GetplayerDistances) (- (Transformation|GetActorLocation _array_element) (Transformation|GetActorLocation))))
  (LocalVariables|SetplayerDistanceSum "0, 0, 0")
  (for _array_element_2 (LocalVariables|GetplayerDistances)
    (LocalVariables|SetplayerDistanceSum (+ (LocalVariables|GetplayerDistanceSum) _array_element_2)))
  ;;[0 0 0] Ensure the net player distance is not greater than the arena's radius
  (LocalVariables|SetplayerDistanceSum (Math|Vector|SelectVector (* (Math|Vector|Normalize (LocalVariables|GetplayerDistanceSum)) _x) (LocalVariables|GetplayerDistanceSum) (> (Math|Vector|VectorLength (LocalVariables|GetplayerDistanceSum)) _x)))
  ;;[0 0 0] Finally update tilt direction and target
  (Variables|Tilt|SettiltDirection (Math|Interpolation|VInterpTo (Variables|Tilt|GettiltDirection) (LocalVariables|GetplayerDistanceSum) (Utilities|Time|GetWorldDeltaSeconds) (Variables|/Game/Systems/Blueprints/GM1/Hazards/Data/PDA_ArenaTilt.PDA_ArenaTilt_C|GetTiltAcceleration (Variables|Tilt|GetArenaTiltData))))
  (Variables|Tilt|SetTargetRotation (Math|Rotator|MakeRotator (* (/ (.Y (Math|Vector|BreakVector (Variables|Tilt|GettiltDirection))) _y) _y_2) (* (/ (.X (Math|Vector|BreakVector (Variables|Tilt|GettiltDirection))) _x_2) _x_3 -1.0) 0.0)))

(fn GetRadiusinUnits
  (bind (_x _y) (Utilities|RadiusinUnits))
  (return _x _y))