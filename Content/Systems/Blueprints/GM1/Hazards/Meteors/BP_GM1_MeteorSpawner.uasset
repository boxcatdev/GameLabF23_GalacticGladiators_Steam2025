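; GM1 hazard spawner that rains meteors onto the arena, either as self-rescheduling random strikes or as single, line, ring and burst patterns.
; Pattern helpers compute points clipped to the arena radius and feed SpawnPattern.
; Each strike attaches a warning AOE zone to the arena, waits a heads-up delay, then launches a meteor down from above, with FX triggered through the game mode's FXManager.
; Construction script previews size and range.
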(event Custom|Stop%20Spawn
  (if (Variables|Default|GetbIsSpawning)
    (Variables|Default|SetbIsSpawning false)
    (for _array_element (Variables|Default|GetcontinuousSpawnTimerHandles)
      (Utilities|Time|ClearandInvalidateTimerbyHandle _array_element))))

(event Custom|Random%20Spawn%20AOE%20Zone%20and%20Meteor
  (if (Variables|Default|GetbIsSpawning)
    (bind _zone (CallFunction|TargetMeteor :meteorSettings (Variables|/Game/Systems/Blueprints/GM1/Hazards/Meteors/Data/PDA_MeteorSpawner.PDA_MeteorSpawner_C|GetMeteor%20Settings (Variables|Default|GetData)) :randomSpawn true))
    ;[0 0 0] Delay before spawning the meteor to give players some heads-up
    (Utilities|FlowControl|Delay (Variables|/Game/Systems/Blueprints/GM1/Hazards/Meteors/Data/PDA_Meteor.PDA_Meteor_C|GetHeads-up%20Time (Variables|/Game/Systems/Blueprints/GM1/Hazards/Meteors/Data/PDA_MeteorSpawner.PDA_MeteorSpawner_C|GetMeteor%20Settings (Variables|Default|GetData))))
    (CallFunction|SpawnMeteorfromTarget (Variables|/Game/Systems/Blueprints/GM1/Hazards/Meteors/Data/PDA_MeteorSpawner.PDA_MeteorSpawner_C|GetMeteor%20Settings (Variables|Default|GetData)) _zone false)
    ;[0 0 0] Spawn another meteor after a delay
    (if (Variables|Default|GetbContinueSpawn)
      (bind _returnvalue (Utilities|Time|SetTimerbyEvent (delegate Custom|Random%20Spawn%20AOE%20Zone%20and%20Meteor) (Utilities|RandomfromRange (Variables|/Game/Systems/Blueprints/GM1/Hazards/Meteors/Data/PDA_MeteorSpawner.PDA_MeteorSpawner_C|GetTarget%20Timer (Variables|Default|GetData)))))
      (Utilities|Array|Add (Variables|Default|GetcontinuousSpawnTimerHandles) _returnvalue))))

(event Custom|Start%20Spawn
  (if (not (Variables|Default|GetbIsSpawning))
    (Variables|Default|SetbIsSpawning true)
    ;[0 0 0] Start spawning meteors after an initial delay
    (Utilities|FlowControl|Delay (Variables|/Game/Systems/Blueprints/GM1/Hazards/Meteors/Data/PDA_MeteorSpawner.PDA_MeteorSpawner_C|GetInitial%20Delay (Variables|Default|GetData)))
    (if (Variables|/Game/Systems/Blueprints/GM1/Hazards/Meteors/Data/PDA_MeteorSpawner.PDA_MeteorSpawner_C|GetAuto%20Start (Variables|Default|GetData))
      (CallFunction|RandomSpawnAOEZoneandMeteor))))

(event Custom|Spawn%20Pattern
  (params (meteorSettings :type PDA%20Meteor%20Object%20Reference) (patternPoints :type Array%20of%20Vector%202D%20Structures))
  ;[0 0 0] Make sure pattern zones is cleared, then put a new AOE zone at each pattern point and save it to pattern zones
  (Utilities|Array|Clear (Variables|Default|GetpatternZones))
  (for _array_element patternPoints
    (bind _zone (CallFunction|TargetMeteor meteorSettings false _array_element (.Value (Utilities|Struct|BreakFloatRangeBound (.UpperBound (Utilities|Struct|BreakFloatRange (Variables|/Game/Systems/Blueprints/GM1/Hazards/Meteors/Data/PDA_Meteor.PDA_Meteor_C|GetSize meteorSettings)))))))
    (Utilities|Array|AddUnique (Variables|Default|GetpatternZones) _zone))
  ;[0 0 0] After a delay, spawn a meteor at each pattern point
  (Utilities|FlowControl|Delay (Variables|/Game/Systems/Blueprints/GM1/Hazards/Meteors/Data/PDA_Meteor.PDA_Meteor_C|GetHeads-up%20Time meteorSettings))
  (for _array_element_2 (Variables|Default|GetpatternZones)
    (CallFunction|SpawnMeteorfromTarget meteorSettings _array_element_2 true)))

(event EventBeginPlay
  ;[0 0 0] Watch for the start of the stage hazards
  (Utilities|Casting|CastToGM_GM1 (Game|GetGameMode)))

(fn ConstructionScript
  (bind _returnvalue (Transformation|GetActorLocation))
  (bind _visual__editor_only_ (Variables|Default|GetVisual%20%28EDITOR%20ONLY%29))
  (bind _data (Variables|Default|GetData))
  (bind _data_2 (Variables|Default|GetData))
  (bind _aoe_range (Variables|/Game/Systems/Blueprints/GM1/Hazards/Meteors/Data/PDA_MeteorSpawner.PDA_MeteorSpawner_C|GetAOE%20Range _data_2))
  (bind _debug_color (Variables|/Game/Systems/Blueprints/GM1/Hazards/Meteors/Data/PDA_MeteorSpawner.PDA_MeteorSpawner_C|GetDebug%20Color _data))
  (bind (_lowerbound _upperbound) (Utilities|Struct|BreakFloatRange _aoe_range))
  (Transformation|SetWorldScale3D _visual__editor_only_ (Math|Conversions|ToVector(Float) (.Value (Utilities|Struct|BreakFloatRangeBound (.LowerBound (Utilities|Struct|BreakFloatRange (Variables|/Game/Systems/Blueprints/GM1/Hazards/Meteors/Data/PDA_Meteor.PDA_Meteor_C|GetSize (Variables|/Game/Systems/Blueprints/GM1/Hazards/Meteors/Data/PDA_MeteorSpawner.PDA_MeteorSpawner_C|GetMeteor%20Settings (Variables|Default|GetData)))))))))
  (Rendering|Components|Decal|SetDecalColor _visual__editor_only_ (Variables|/Game/Systems/Blueprints/GM1/Hazards/Meteors/Data/PDA_MeteorSpawner.PDA_MeteorSpawner_C|GetAOE%20Color _data_2))
  (Rendering|Debug|DrawDebugCircle _returnvalue (.Value (Utilities|Struct|BreakFloatRangeBound _lowerbound)) 32 _debug_color 1.0 5.0 "0.000000,1.000000,0.000000" "1.000000,0.000000,0.000000")
  (Rendering|Debug|DrawDebugCircle _returnvalue (.Value (Utilities|Struct|BreakFloatRangeBound _upperbound)) 32 _debug_color 1.0 5.0 "0.000000,1.000000,0.000000" "1.000000,0.000000,0.000000"))

(fn TargetMeteor
  (params (meteorSettings :type PDA%20Meteor%20Object%20Reference) (randomSpawn :type Boolean) (setPosition :type Vector%202D%20Structure) (setSize :type Float%20%28double-precision%29))
  (bind _returnvalue (Transformation|GetActorLocation))
  (bind _returnvalue_2 (Game|GetGameInstance))
  (bind _returnvalue_3 (Transformation|GetActorLocation))
  (bind _data (Variables|Default|GetData))
  (bind _returnvalue_4 (+ _returnvalue setPosition))
  (bind _aoe_range (Variables|/Game/Systems/Blueprints/GM1/Hazards/Meteors/Data/PDA_MeteorSpawner.PDA_MeteorSpawner_C|GetAOE%20Range _data))
  (bind _value (Utilities|RandomfromRange _aoe_range))
  (bind _vector (Utilities|RandomVector _returnvalue_2 _value))
  (bind _returnvalue_5 (+ _returnvalue_3 _vector))
  (bind _returnvalue_6 (Math|Vector|SelectVector _returnvalue_5 _returnvalue_4 randomSpawn))
  (bind (_x _y) (Class|KismetMathLibrary|BreakVector3f _returnvalue_6))
  (bind _returnvalue_7 (Actor|GetActorOfClass "/Game/Systems/Blueprints/GM1/Hazards/BP_Arena.BP_Arena_C"))
  ;[0 0 0 0.5] Spawn an AOEZone, and parent it to the arena floor
  (bind _returnvalue_8 (Game|SpawnActorfromClass "/Game/Systems/Blueprints/GM1/Hazards/Meteors/BP_GM1_AOEZone.BP_GM1_AOEZone_C" (Math|Transform|MakeTransform (Math|Vector|MakeVector _x _y (+ (.z (Transformation|GetWorldLocation (Variables|/Game/Systems/Blueprints/GM1/Hazards/BP_Arena.BP_Arena_C|GetArena%20Floor _returnvalue_7))) 5.0)) "0, 0, 0" (Math|Vector|SelectVector (Math|Conversions|ToVector(Float) (Utilities|RandomfromRange (Variables|/Game/Systems/Blueprints/GM1/Hazards/Meteors/Data/PDA_Meteor.PDA_Meteor_C|GetSize meteorSettings))) (Math|Conversions|ToVector(Float) setSize) randomSpawn)) "AlwaysSpawn" "MultiplyWithRoot" 0 0))
  (Transformation|AttachActorToActor _returnvalue_8 _returnvalue_7 "None" "KeepWorld" "KeepWorld" "KeepWorld" true)
  (Default|SetParticles _returnvalue_8 meteorSettings)
  (bind _asgm_gm1 (Utilities|Casting|CastToGM_GM1 (Game|GetGameMode)))
  (if (Variables|/Game/Systems/Blueprints/GM1/Hazards/Meteors/Data/PDA_Meteor.PDA_Meteor_C|GetUseLargeFX meteorSettings)
    (Default|CallGM1HazardLargeMeteorTarget (Variables|/Game/Systems/Blueprints/GM1/Systems/GM_GM1.GM_GM1_C|GetFXManager _asgm_gm1) _returnvalue_8)
    (else
      (Default|CallGM1HazardMeteorTarget (Variables|/Game/Systems/Blueprints/GM1/Systems/GM_GM1.GM_GM1_C|GetFXManager _asgm_gm1) _returnvalue_8)))
  (return _returnvalue_8))

(fn SpawnMeteorfromTarget
  (params (meteorSettings :type PDA%20Meteor%20Object%20Reference) (AOE%20Zone :type BP%20GM1%20AOE%20Zone%20Object%20Reference) (bIsPattern :type Boolean))
  (bind _returnvalue (Transformation|GetActorLocation AOE%20Zone))
  (bind _speed (Variables|/Game/Systems/Blueprints/GM1/Hazards/Meteors/Data/PDA_Meteor.PDA_Meteor_C|GetSpeed meteorSettings))
  (Utilities|IsValid AOE%20Zone
    (:Is%20Valid
      (bind _returnvalue_2 (Game|SpawnActorfromClass (Variables|/Game/Systems/Blueprints/GM1/Hazards/Meteors/Data/PDA_Meteor.PDA_Meteor_C|GetType meteorSettings) (Class|KismetAnimationLibrary|Lookat (Math|Transform|MakeTransform (+ _returnvalue (Math|Vector|MakeVector 0.0 0.0 (Variables|Default|GetspawnHeight))) "0, 0, 0" (Math|Conversions|ToVector(Float) (Variables|/Game/Systems/Blueprints/GM1/Hazards/Meteors/BP_GM1_AOEZone.BP_GM1_AOEZone_C|GettargetSize AOE%20Zone))) _returnvalue "1.000000,0.000000,0.000000" false "0, 0, 0" 0.0) "AlwaysSpawn" "MultiplyWithRoot" 0 0))
      (bind _output_get (Variables|/Game/Systems/Blueprints/GM1/Hazards/Meteors/BP_GM1_AOEZone.BP_GM1_AOEZone_C|SetwatchMeteor AOE%20Zone _returnvalue_2))
      (Default|ApplyMeteorSettings _output_get meteorSettings AOE%20Zone)
      (Physics|AddImpulse (Variables|/Game/Systems/Blueprints/GM1/Hazards/Meteors/BP_GM1_Meteor.BP_GM1_Meteor_C|GetSphereCol _returnvalue_2) (* "0.000000,0.000000,-1.000000" (Math|Float|SelectFloat (.Value (Utilities|Struct|BreakFloatRangeBound (.UpperBound (Utilities|Struct|BreakFloatRange _speed)))) (Utilities|RandomfromRange _speed) bIsPattern)) "None" true)
      (bind _asgm_gm1 (Utilities|Casting|CastToGM_GM1 (Game|GetGameMode)))
      (if (Variables|/Game/Systems/Blueprints/GM1/Hazards/Meteors/Data/PDA_Meteor.PDA_Meteor_C|GetUseLargeFX meteorSettings)
        (Default|CallGM1HazardLargeMeteorSpawn (Variables|/Game/Systems/Blueprints/GM1/Systems/GM_GM1.GM_GM1_C|GetFXManager _asgm_gm1) _returnvalue_2)
        (else
          (Default|CallGM1HazardMeteorSpawn (Variables|/Game/Systems/Blueprints/GM1/Systems/GM_GM1.GM_GM1_C|GetFXManager _asgm_gm1) _returnvalue_2)))
      (return _returnvalue_2))))

(fn CalculateLine
  (params (p1 :type Vector%202D%20Structure) (p2 :type Vector%202D%20Structure) (width :type Float%20%28double-precision%29) (vertices :type Integer))
  (bind _returnvalue (- vertices 1))
  (bind _returnvalue_2 (Actor|GetActorOfClass "/Game/Systems/Blueprints/GM1/Hazards/BP_Arena.BP_Arena_C"))
  (bind _output_get (LocalVariables|Setarena _returnvalue_2))
  (bind _x (Default|GetRadiusinUnits _output_get))
  (LocalVariables|SetarenaRadius _x)
  (for _index (range 0 _returnvalue)
    (if (<= (Math|Vector2D|Vector2DLength (+ (* (/ (Math|Conversions|ToFloat(Integer) _index) (Math|Conversions|ToFloat(Integer) _returnvalue)) (- p2 p1)) p1)) (LocalVariables|GetarenaRadius))
      (Utilities|Array|AddUnique (LocalVariables|GetlinePoints) (+ (* (/ (Math|Conversions|ToFloat(Integer) _index) (Math|Conversions|ToFloat(Integer) _returnvalue)) (- p2 p1)) p1))))
  (return (LocalVariables|GetlinePoints)))

(fn CalculateRing
  (params (center :type Vector%202D%20Structure) (radius :type Float%20%28double-precision%29) (numPoints :type Integer))
  (bind _returnvalue (Actor|GetActorOfClass "/Game/Systems/Blueprints/GM1/Hazards/BP_Arena.BP_Arena_C"))
  (bind _output_get (LocalVariables|Setarena _returnvalue))
  (bind _x (Default|GetRadiusinUnits _output_get))
  (LocalVariables|SetarenaRadius _x)
  (for _index (range 0 (- numPoints 1))
    ;[0 0 0] Get the point of the ring at the current angle
    (bind _output_get_2 (LocalVariables|Setcurrent (+ center (* (Math|Vector2D|MakeVector2D (Math|Trig|Cos(Degrees) (* _index (/ 3.6e+02 (Math|Conversions|ToFloat(Integer) numPoints)))) (Math|Trig|Sin(Degrees) (* _index (/ 3.6e+02 (Math|Conversions|ToFloat(Integer) numPoints))))) radius))))
    ;[0 0 0] If the new point is in the bounds of the arena, add it to the list pf points
    (if (< (Math|Vector2D|Vector2DLength _output_get_2) (LocalVariables|GetarenaRadius))
      (Utilities|Array|AddUnique (LocalVariables|GetringPoints) (LocalVariables|Getcurrent))))
  (return (LocalVariables|GetringPoints)))

(fn CalculateBurst
  (params (center :type Vector%202D%20Structure) (radius :type Float%20%28double-precision%29) (numPoints :type Integer))
  (bind _returnvalue (Actor|GetActorOfClass "/Game/Systems/Blueprints/GM1/Hazards/BP_Arena.BP_Arena_C"))
  (bind _output_get (LocalVariables|Setarena _returnvalue))
  (bind _x (Default|GetRadiusinUnits _output_get))
  (LocalVariables|SetarenaRadius _x)
  (for _index (range 0 (- numPoints 1))
    ;[0 0 0 0.25] Similar to CalculateRing except that it uses a random radius rather than a set one
    ;;[0 0 0] Get a point at a random distance from the center of the circle along the current angle
    (bind _output_get_2 (LocalVariables|Setcurrent (+ center (* (Math|Vector2D|MakeVector2D (Math|Trig|Cos(Degrees) (* _index (/ 3.6e+02 (Math|Conversions|ToFloat(Integer) numPoints)))) (Math|Trig|Sin(Degrees) (* _index (/ 3.6e+02 (Math|Conversions|ToFloat(Integer) numPoints))))) (Utilities|RandomFloat (Game|GetGameInstance) radius)))))
    ;;[0 0 0] If the new point is in the bounds of the arena, add it to the list pf points
    (if (< (Math|Vector2D|Vector2DLength _output_get_2) (LocalVariables|GetarenaRadius))
      (Utilities|Array|AddUnique (LocalVariables|GetburstPoints) (LocalVariables|Getcurrent))))
  (return (LocalVariables|GetburstPoints)))

(fn SpawnMeteorSingle
  (params (meteorSettings :type PDA%20Meteor%20Object%20Reference) (position :type Vector%202D%20Structure))
  (CallFunction|SpawnPattern meteorSettings (Utilities|Array|MakeArray position)))

(fn SpawnMeteorLine
  (params (meteorSettings :type PDA%20Meteor%20Object%20Reference) (p1 :type Vector%202D%20Structure) (p2 :type Vector%202D%20Structure) (vertices :type Integer))
  (bind _points (MeteorPatterns|CalculateLine p1 p2 (.Value (Utilities|Struct|BreakFloatRangeBound (.UpperBound (Utilities|Struct|BreakFloatRange (Variables|/Game/Systems/Blueprints/GM1/Hazards/Meteors/Data/PDA_Meteor.PDA_Meteor_C|GetSize meteorSettings))))) vertices))
  (CallFunction|SpawnPattern meteorSettings _points))

(fn SpawnMeteorRing
  (params (meteorSettings :type PDA%20Meteor%20Object%20Reference) (position :type Vector%202D%20Structure) (radius :type Float%20%28double-precision%29) (points :type Integer))
  (bind _points (MeteorPatterns|CalculateRing position radius points))
  (CallFunction|SpawnPattern meteorSettings _points))

(fn SpawnMeteorBurst
  (params (meteorSettings :type PDA%20Meteor%20Object%20Reference) (position :type Vector%202D%20Structure) (radius :type Float%20%28double-precision%29) (count :type Integer))
  (bind _points (MeteorPatterns|CalculateBurst position radius count))
  (CallFunction|SpawnPattern meteorSettings _points))