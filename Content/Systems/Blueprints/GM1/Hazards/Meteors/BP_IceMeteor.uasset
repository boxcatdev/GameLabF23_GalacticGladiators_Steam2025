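; BP_IceMeteor is a meteor hazard variant that leaves an ice patch on the arena floor where it lands.
; It extends the parent Impact to spawn BP_IcePatch at floor height with random yaw and radius-based scale, then attaches it to BP_Arena.
; InitializeTrail pulls the trail effect from the game instance's GM1 VFX atlas and activates it with a flipped rotation.
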(event EventBeginPlay
  (|CallParentFunction) ; This node is disabled and will not be called.\nDrag off pins to build functionality.
)

(event Collision|EventActorBeginOverlap
  (params (OtherActor :type Actor%20Object%20Reference))
  (|CallParentFunction OtherActor) ; This node is disabled and will not be called.\nDrag off pins to build functionality.
)

(event EventTick
  (params (DeltaSeconds :type Float%20%28single-precision%29))
  (|CallParentFunction DeltaSeconds) ; This node is disabled and will not be called.\nDrag off pins to build functionality.
)

(fn ConstructionScript
  (|CallParentFunction))

(fn Impact
  (bind _returnvalue (Transformation|GetActorLocation))
  (|CallParentFunction)
  ;[0 0 0] Spawn an ice patch at the meteor's transform, making sure it is parented to the arena floor correctly
  (bind _returnvalue_2 (Actor|GetActorOfClass "/Game/Systems/Blueprints/GM1/Hazards/BP_Arena.BP_Arena_C"))
  (LocalVariables|Setarena _returnvalue_2)
  (bind _returnvalue_3 (Game|SpawnActorfromClass "/Game/Systems/Blueprints/GM1/Hazards/BP_IcePatch.BP_IcePatch_C" (Math|Transform|MakeTransform (Math|Vector|MakeVector (.x _returnvalue) (.y _returnvalue) (.z (Transformation|GetWorldLocation (Variables|/Game/Systems/Blueprints/GM1/Hazards/BP_Arena.BP_Arena_C|GetArena%20Floor (LocalVariables|Getarena))))) (Math|Rotator|MakeRotator 0.0 0.0 (Math|Random|RandomFloatinRange 0.0 3.6e+02)) (Math|Conversions|ToVector(Float) (/ (Variables|Default|GetRadius) 5e+01))) "Undefined" "MultiplyWithRoot" 0 0))
  (Transformation|AttachActorToActor _returnvalue_3 (LocalVariables|Getarena) "None" "KeepWorld" "KeepWorld" "KeepRelative" true))

(fn InitializeTrail
  (bind _trailparticles (Variables|Default|GetTrailParticles))
  (bind _asgi_core_game_instance (Utilities|Casting|CastToGI_CORE_GameInstance (Game|GetGameInstance)))
  (Class|NiagaraComponent|SetAsset _trailparticles (.Value (Utilities|Map|Find (Variables|/Game/Core/Programming/Prototypes/Test_Sai/PDA_VFX_GM1_Atlas.PDA_VFX_GM1_Atlas_C|GetVFXAssets (Variables|/Game/Core/Programming/Prototypes/GameData/GI_CORE_GameInstance.GI_CORE_GameInstance_C|GetGM1VFXAtlas _asgi_core_game_instance)) "NewEnumerator7")) true)
  (Components|Activation|Activate _trailparticles false)
  (Transformation|SetWorldRotation _trailparticles "0.000000,0.000000,180.000000" false false))