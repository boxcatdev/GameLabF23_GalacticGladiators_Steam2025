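; BP_GM1_AOEZone is the ground zone marker for GM1 meteor hazards, with particles matched to the meteor type.
; On spawn a timeline scales it up to its placed size, and SetParticles picks an ice or default effect from the game instance's VFX atlas.
; Tick stops tracking the watched meteor once it is hidden; the decal flash and fade-out-destroy logic is disconnected.
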(event EventBeginPlay
  ;[0 0 0] Animate Scale Intro
  (Variables|Default|SettargetSize (.X (Math|Vector|BreakVector (Transformation|GetActorScale3D))))
  (bind _scale (Timeline|SizeAnim PlayFromStart)
    (:Update
      (Transformation|SetActorScale3D (Math|Conversions|ToVector(Float) (* _scale (Variables|Default|GettargetSize)))))))

(event EventTick
  (params (DeltaSeconds :type Float%20%28single-precision%29))
  (Utilities|IsValid (Variables|Default|GetwatchMeteor)
    (:Is%20Valid
      (if (Variables|/Script/Engine.Actor|GetbHidden (Variables|Default|GetwatchMeteor))
        ;[0 0 0] Hazard was destroyed, setup Fade Out auto destroy
        (Variables|Default|SetcheckingForHazard false)
        (Variables|Default|SetwatchMeteor 0)))))

(fn ConstructionScript)

(fn SetParticles
  (params (settings :type PDA%20Meteor%20Object%20Reference))
  (bind _targetparticles (Variables|Default|GetTargetParticles))
  (bind _asgi_core_game_instance (Utilities|Casting|CastToGI_CORE_GameInstance (Game|GetGameInstance)))
  (Class|NiagaraComponent|SetAsset _targetparticles (.Value (Utilities|Map|Find (Variables|/Game/Core/Programming/Prototypes/Test_Sai/PDA_VFX_GM1_Atlas.PDA_VFX_GM1_Atlas_C|GetVFXAssets (Variables|/Game/Core/Programming/Prototypes/GameData/GI_CORE_GameInstance.GI_CORE_GameInstance_C|GetGM1VFXAtlas _asgi_core_game_instance)) (select (== (Variables|/Game/Systems/Blueprints/GM1/Hazards/Meteors/Data/PDA_Meteor.PDA_Meteor_C|GetType settings) "/Game/Systems/Blueprints/GM1/Hazards/Meteors/BP_IceMeteor.BP_IceMeteor_C") (Utilities|Enum|LiteralenumE_GM1_VFXEvents "NewEnumerator17") (Utilities|Enum|LiteralenumE_GM1_VFXEvents "NewEnumerator16")))) true)
  (Components|Activation|Activate _targetparticles false))