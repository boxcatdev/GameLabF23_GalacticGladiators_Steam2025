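; GM1 meteor hazard actor, configured with settings and a target zone that sets its blast radius, with a trail effect from the game instance's VFX atlas.
; On overlapping the arena it applies a manual radial impulse, optionally horizontal-only, to players and static mesh actors, also stunning players and making them drop crowns.
; It then triggers small or large impact FX through the game mode and destroys itself and its target.
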(event EventDestroyed
  (bind _target (Variables|Default|Gettarget))
  (Utilities|IsValid _target
    (:Is%20Valid
      (Actor|DestroyActor _target))))

(event EventBeginPlay
  ;[1 0.5706 0] Should be overridden in child classes
  (CallFunction|InitializeTrail)
  (Utilities|FlowControl|DelayUntilNextTick)
  (Variables|Default|SetrotSpeedVector (* (Math|Random|RandomUnitVector) (Variables|/Game/Systems/Blueprints/GM1/Hazards/Meteors/Data/PDA_Meteor.PDA_Meteor_C|GetRotational%20Speed (Variables|Default|GetSettings))))
  (Transformation|SetRelativeRotation (Variables|Default|GetMesh) (Math|Random|RandomRotator true) false false))

(event EventTick
  (params (DeltaSeconds :type Float%20%28single-precision%29))
  (Transformation|AddRelativeRotation (Variables|Default|GetMesh) (Math|Conversions|RotationFromXVector (* (Variables|Default|GetrotSpeedVector) "")) false false))

(event Collision|EventActorBeginOverlap
  (params (OtherActor :type Actor%20Object%20Reference))
  (Utilities|Casting|CastToBP_Arena OtherActor)
  (Physics|SetPhysicsLinearVelocity (Variables|Default|GetSphereCol) "0, 0, 0" false "None")
  (CallFunction|Impact))

(fn ConstructionScript)

(fn Impact
  (bind _returnvalue (Transformation|GetActorLocation))
  (bind _self self)
  ;[0 0 0] Knock back each actor in the radius of effect. Effectively apes a RadialForceComponent except that we can fix the impulse to the horizontal.
  (bind _outactors (Collision|SphereOverlapActors _returnvalue (Variables|Default|GetRadius) (Variables|Default|GetAffect%20Channels) 0))
  (for _array_element _outactors
    (bind _asbp_player_gm1 (Utilities|Casting|CastToBP_Player_GM1 _array_element)
      (:then
        (Default|AddImpulse _asbp_player_gm1 (* (Math|Vector|SelectVector (Class|KismetMathLibrary|VectorNormal2D (- (Transformation|GetActorLocation _array_element) _returnvalue) 0.0001) (Math|Vector|Normalize (- (Transformation|GetActorLocation _array_element) _returnvalue)) (Variables|/Game/Systems/Blueprints/GM1/Hazards/Meteors/Data/PDA_Meteor.PDA_Meteor_C|GetHorizontal%20Impulse%20Only (Variables|Default|GetSettings))) (Utilities|GetMeteorForcefromSize (Variables|Default|GetRadius))) false)
        (Default|DropCrown _asbp_player_gm1 self)
        (Default|ApplyStun _asbp_player_gm1 (Variables|/Game/Systems/Blueprints/GM1/Hazards/Meteors/Data/PDA_Meteor.PDA_Meteor_C|GetStun%20Time (Variables|Default|GetSettings))))
      (:CastFailed
        (bind _asstatic_mesh_actor (Utilities|Casting|CastToStaticMeshActor _array_element))
        (Physics|AddImpulse (Variables|/Script/Engine.StaticMeshActor|GetStaticMeshComponent _asstatic_mesh_actor) (* (Math|Vector|SelectVector (Class|KismetMathLibrary|VectorNormal2D (- (Transformation|GetActorLocation _array_element) _returnvalue) 0.0001) (Math|Vector|Normalize (- (Transformation|GetActorLocation _array_element) _returnvalue)) (Variables|/Game/Systems/Blueprints/GM1/Hazards/Meteors/Data/PDA_Meteor.PDA_Meteor_C|GetHorizontal%20Impulse%20Only (Variables|Default|GetSettings))) (Utilities|GetMeteorForcefromSize (Variables|Default|GetRadius))) "None" false))))
  (bind _asgm_gm1 (Utilities|Casting|CastToGM_GM1 (Game|GetGameMode)))
  (if (Variables|/Game/Systems/Blueprints/GM1/Hazards/Meteors/Data/PDA_Meteor.PDA_Meteor_C|GetUseLargeFX (Variables|Default|GetSettings))
    (Default|CallGM1HazardLargeMeteorImpact (Variables|/Game/Systems/Blueprints/GM1/Systems/GM_GM1.GM_GM1_C|GetFXManager _asgm_gm1) _self)
    (else
      (Default|CallGM1HazardMeteorImpact (Variables|/Game/Systems/Blueprints/GM1/Systems/GM_GM1.GM_GM1_C|GetFXManager _asgm_gm1) _self)))
  (Actor|DestroyActor))

(fn ApplyMeteorSettings
  (params (settings :type PDA%20Meteor%20Object%20Reference) (targetZone :type BP%20GM1%20AOE%20Zone%20Object%20Reference))
  (Variables|Default|SetSettings settings)
  (Variables|Default|Settarget targetZone)
  (Variables|Default|SetRadius (* (Variables|/Game/Systems/Blueprints/GM1/Hazards/Meteors/BP_GM1_AOEZone.BP_GM1_AOEZone_C|GettargetSize targetZone) 5e+01)))

(fn InitializeTrail
  (bind _trailparticles (Variables|Default|GetTrailParticles))
  (bind _asgi_core_game_instance (Utilities|Casting|CastToGI_CORE_GameInstance (Game|GetGameInstance)))
  (Class|NiagaraComponent|SetAsset _trailparticles (.Value (Utilities|Map|Find (Variables|/Game/Core/Programming/Prototypes/Test_Sai/PDA_VFX_GM1_Atlas.PDA_VFX_GM1_Atlas_C|GetVFXAssets (Variables|/Game/Core/Programming/Prototypes/GameData/GI_CORE_GameInstance.GI_CORE_GameInstance_C|GetGM1VFXAtlas _asgi_core_game_instance)) "NewEnumerator6")) true)
  (Components|Activation|Activate _trailparticles false)
  (Transformation|SetWorldRotation _trailparticles "0.000000,0.000000,180.000000" false false))