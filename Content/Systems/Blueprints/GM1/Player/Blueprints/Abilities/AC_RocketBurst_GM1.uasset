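; Player ability component for GM1: a rocket dash that rams players and objects, stealing the crown on a hit.
; Looping timers drive velocity from a speed curve and sphere-trace for impacts, then a cooldown ends with a recharge flash.
; Hits launch and stun the victim, or repel both players if both dash; crown carriers trigger an area stun.
; Every impact radially knocks back nearby players and movable meshes, optionally horizontal-only.
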(event Custom|TryAbilityRocketBurst
  (if (Utilities|CanRocketBurst)
    (CallFunction|StartRocketBurst)))

(event Custom|ClearCooldown
  (Variables|Default|SetbIsOnCooldown false)
  (bind _asgm_gm1 (Utilities|Casting|CastToGM_GM1 (Game|GetGameMode)))
  (Default|CallGM1PlayerRocketBurstRecharged (Variables|/Game/Systems/Blueprints/GM1/Systems/GM_GM1.GM_GM1_C|GetFXManager _asgm_gm1) (Variables|Default|GetPlayer))
  (Default|CallOnCooldown)
  (CallFunction|SetFlash (Variables|Default|GetPlayer) true)
  (Utilities|FlowControl|Delay 0.2)
  (CallFunction|SetFlash (Variables|Default|GetPlayer) false))

(event EventBeginPlay
  (|CallParentFunction) ; This node is disabled and will not be called.\nDrag off pins to build functionality.
)

(fn StartRocketBurst
  (Variables|Default|SetbIsDashing true)
  (bind _returnvalue (Utilities|Time|SetTimerbyFunctionName 0 "DashUpdate" (Variables|Default|GetupdateStep) true))
  (Variables|TimerHandles|SetUpdateHandle _returnvalue)
  (bind _returnvalue_2 (Utilities|Time|SetTimerbyFunctionName 0 "EndRocketBurst" (Variables|/Game/Systems/Blueprints/GM1/Player/Systems/Data/PDA_RocketBurst.PDA_RocketBurst_C|GetDuration (Variables|Default|GetRocketBurstData))))
  (Variables|TimerHandles|SetActiveTimerHandle _returnvalue_2)
  (Default|CallOnRocketBurst self)
  (bind _asgm_gm1 (Utilities|Casting|CastToGM_GM1 (Game|GetGameMode)))
  (Default|CallGM1PlayerRocketBurstStarted (Variables|/Game/Systems/Blueprints/GM1/Systems/GM_GM1.GM_GM1_C|GetFXManager _asgm_gm1) (Variables|Default|GetPlayer)))

(fn DashUpdate
  (Variables|/Script/Engine.MovementComponent|SetVelocity (Variables|Default|GetCharacter%20Movement) (* (Transformation|GetActorForwardVector (Variables|Default|GetPlayer)) (Utilities|GetDashSpeedThisFrame)))
  (CallFunction|CheckImpact))

(fn EndRocketBurst
  (Variables|Default|SetbIsDashing false)
  (Variables|Default|SetbIsOnCooldown true)
  (Utilities|Time|ClearandInvalidateTimerbyHandle (Variables|TimerHandles|GetUpdateHandle))
  (Utilities|Time|ClearandInvalidateTimerbyHandle (Variables|TimerHandles|GetActiveTimerHandle))
  (bind _returnvalue (Utilities|Time|SetTimerbyFunctionName 0 "ClearCooldown" (Variables|/Game/Systems/Blueprints/GM1/Player/Systems/Data/PDA_RocketBurst.PDA_RocketBurst_C|GetCooldown (Variables|Default|GetRocketBurstData))))
  (Variables|TimerHandles|SetCooldownTimerHandle _returnvalue))

(fn CheckImpact
  (bind _player (Variables|Default|GetPlayer))
  (bind _rocketburstdata (Variables|Default|GetRocketBurstData))
  (bind _returnvalue (Transformation|GetActorForwardVector _player))
  (bind _returnvalue_2 (Transformation|GetActorLocation _player))
  (bind _hitrange (Variables|/Game/Systems/Blueprints/GM1/Player/Systems/Data/PDA_RocketBurst.PDA_RocketBurst_C|GetHitRange _rocketburstdata))
  (bind _returnvalue_3 (* _returnvalue _hitrange))
  (bind _returnvalue_4 (+ _returnvalue_2 _returnvalue_3))
  (bind _outactors (Actor|GetAllActorsOfClass "/Game/Systems/Blueprints/GM1/Hazards/BP_Arena.BP_Arena_C"))
  (bind _outhit (Collision|SphereTraceByChannel _returnvalue_4 _returnvalue_4 (Variables|/Game/Systems/Blueprints/GM1/Player/Systems/Data/PDA_RocketBurst.PDA_RocketBurst_C|GetHitRadius _rocketburstdata) "TraceTypeQuery1" false _outactors "None" true "(R=1.000000,G=0.000000,B=0.000000,A=0.000000)" "(R=0.000000,G=1.000000,B=0.000000,A=1.000000)" 0.5))
  (if (.bBlockingHit (Collision|BreakHitResult _outhit))
    (bind _asbp_player_gm1 (Utilities|Casting|CastToBP_Player_GM1 (.HitActor (Collision|BreakHitResult _outhit)))
      (:then
        (CallFunction|ImpactPlayer _asbp_player_gm1))
      (:CastFailed
        (CallFunction|ImpactObject)))
    (CallFunction|EndRocketBurst)
    (bind _asgm_gm1 (Utilities|Casting|CastToGM_GM1 (Game|GetGameMode)))
    (Default|CallGM1PlayerRocketBurstImpact (Variables|/Game/Systems/Blueprints/GM1/Systems/GM_GM1.GM_GM1_C|GetFXManager _asgm_gm1) (Variables|Default|GetPlayer) (.Location (Collision|BreakHitResult _outhit)))
    (Rendering|Debug|DrawDebugSphere (Transformation|GetActorLocation (Variables|Default|GetPlayer)) 1e+02 12 "(R=1.000000,G=0.647319,B=0.000000,A=1.000000)" 0.5 2.0)))

(fn ImpactPlayer
  (params (hit :type BP%20Player%20GM1%20Object%20Reference))
  (bind _rocketburstdata (Variables|Default|GetRocketBurstData))
  (bind _rocketburstdata_2 (Variables|Default|GetRocketBurstData))
  (bind _bhascrown (Variables|/Game/Systems/Blueprints/GM1/Player/Blueprints/BP_Player_GM1.BP_Player_GM1_C|GetbHasCrown hit))
  (bind _impactscale (Variables|/Game/Systems/Blueprints/GM1/Player/Systems/Data/PDA_RocketBurst.PDA_RocketBurst_C|GetImpactScale _rocketburstdata_2))
  (bind _crownstealimpactscale (Variables|/Game/Systems/Blueprints/GM1/Player/Systems/Data/PDA_RocketBurst.PDA_RocketBurst_C|GetCrownStealImpactScale _rocketburstdata_2))
  (bind _returnvalue (Math|Float|SelectFloat _crownstealimpactscale _impactscale _bhascrown))
  (if (Variables|/Game/Systems/Blueprints/GM1/Player/Blueprints/BP_Player_GM1.BP_Player_GM1_C|GetbHasCrown hit)
    (CallFunction|RadialStun (Utilities|Array|MakeArray (Variables|Default|GetPlayer)) (Variables|/Game/Systems/Blueprints/GM1/Player/Systems/Data/PDA_RocketBurst.PDA_RocketBurst_C|GetCrownStealRadius _rocketburstdata) (Variables|/Game/Systems/Blueprints/GM1/Player/Systems/Data/PDA_RocketBurst.PDA_RocketBurst_C|GetCrownStealStunDuration _rocketburstdata)))
  (if (Variables|AC_RocketBurst_GM1_C|GetbIsDashing (Variables|/Game/Systems/Blueprints/GM1/Player/Blueprints/BP_Player_GM1.BP_Player_GM1_C|GetAC_RocketBurst hit))
    (CallFunction|LaunchBothPlayers hit _returnvalue)
    (else
      (CallFunction|LaunchPlayer hit (Math|Float|SelectFloat (Variables|/Game/Systems/Blueprints/GM1/Player/Systems/Data/PDA_RocketBurst.PDA_RocketBurst_C|GetCrownStealStunDuration _rocketburstdata_2) (Variables|/Game/Systems/Blueprints/GM1/Player/Systems/Data/PDA_RocketBurst.PDA_RocketBurst_C|GetStunDuration _rocketburstdata_2) _bhascrown) _returnvalue)))
  (CallFunction|RadialLaunch (Utilities|Array|MakeArray hit (Variables|Default|GetPlayer)) (Math|Float|SelectFloat (Variables|/Game/Systems/Blueprints/GM1/Player/Systems/Data/PDA_RocketBurst.PDA_RocketBurst_C|GetCrownStealRadius _rocketburstdata_2) (Variables|/Game/Systems/Blueprints/GM1/Player/Systems/Data/PDA_RocketBurst.PDA_RocketBurst_C|GetRadius _rocketburstdata_2) _bhascrown) (Math|Float|SelectFloat (Variables|/Game/Systems/Blueprints/GM1/Player/Systems/Data/PDA_RocketBurst.PDA_RocketBurst_C|GetCrownStealRadialForce _rocketburstdata_2) (Variables|/Game/Systems/Blueprints/GM1/Player/Systems/Data/PDA_RocketBurst.PDA_RocketBurst_C|GetRadialForce _rocketburstdata_2) _bhascrown))
  (Default|CallOnImpulseReceived hit (Variables|Default|GetPlayer)))

(fn ImpactObject
  (bind _rocketburstdata (Variables|Default|GetRocketBurstData))
  (CallFunction|RadialLaunch (Utilities|Array|MakeArray (Variables|Default|GetPlayer)) (Variables|/Game/Systems/Blueprints/GM1/Player/Systems/Data/PDA_RocketBurst.PDA_RocketBurst_C|GetRadius _rocketburstdata) (Variables|/Game/Systems/Blueprints/GM1/Player/Systems/Data/PDA_RocketBurst.PDA_RocketBurst_C|GetRadialForce _rocketburstdata)))

(fn LaunchPlayer
  (params (launch :type BP%20Player%20GM1%20Object%20Reference) (stunDuration :type Float%20%28double-precision%29) (impactScale :type Float%20%28double-precision%29))
  (bind _character_movement (Variables|Default|GetCharacter%20Movement))
  (bind _player (Variables|Default|GetPlayer))
  (LocalVariables|SetlaunchVelocity (Variables|/Script/Engine.MovementComponent|GetVelocity _character_movement))
  (Variables|/Script/Engine.MovementComponent|SetVelocity _character_movement "0, 0, 0")
  (Default|AddImpulse launch (* (LocalVariables|GetlaunchVelocity) impactScale) true)
  (Default|ApplyStun launch stunDuration)
  (Default|DropCrown launch _player _player))

(fn LaunchBothPlayers
  (params (other :type BP%20Player%20GM1%20Object%20Reference) (impactScale :type Float%20%28double-precision%29))
  (bind _player (Variables|Default|GetPlayer))
  (bind _returnvalue (Transformation|GetActorLocation _player))
  (bind _returnvalue_2 (Transformation|GetActorLocation other))
  (LocalVariables|SetimpactSpeed (* (Math|Vector|VectorLength (- (Variables|/Script/Engine.MovementComponent|GetVelocity (Variables|Default|GetCharacter%20Movement)) (Variables|/Script/Engine.MovementComponent|GetVelocity (Variables|/Script/Engine.Character|GetCharacterMovement other)))) impactScale 0.5))
  (bind _output_get (LocalVariables|SetplayerVelocityNew (* (Math|Vector|Normalize (- _returnvalue _returnvalue_2)) (LocalVariables|GetimpactSpeed))))
  (bind _output_get_2 (LocalVariables|SetotherVelocityNew (* (Math|Vector|Normalize (- _returnvalue_2 _returnvalue)) (LocalVariables|GetimpactSpeed))))
  (Default|AddImpulse (Variables|Default|GetPlayer) _output_get true)
  (Default|AddImpulse other _output_get_2 true)
  (CallFunction|EndRocketBurst (Variables|/Game/Systems/Blueprints/GM1/Player/Blueprints/BP_Player_GM1.BP_Player_GM1_C|GetAC_RocketBurst other)))

(fn RadialLaunch
  (params (ignorePlayers :type Array%20of%20Actor%20Object%20References) (radius :type Float%20%28double-precision%29) (force :type Float%20%28double-precision%29))
  (bind _rocketburstdata (Variables|Default|GetRocketBurstData))
  (bind _player (Variables|Default|GetPlayer))
  (bind _returnvalue (Transformation|GetActorLocation _player))
  ;[0 0 0] Knock back each actor in the radius of effect. Effectively apes a RadialForceComponent except that we can fix the impulse to the horizontal.
  (bind _outactors (Collision|SphereOverlapActors _returnvalue radius (Variables|Default|GetRadialLaunchChannels) 0 ignorePlayers))
  (for _array_element _outactors
    (bind _asbp_player_gm1 (Utilities|Casting|CastToBP_Player_GM1 _array_element)
      (:then
        (Default|AddImpulse _asbp_player_gm1 (* (Math|Vector|SelectVector (Class|KismetMathLibrary|VectorNormal2D (- (Transformation|GetActorLocation _array_element) _returnvalue) 0.0001) (Math|Vector|Normalize (- (Transformation|GetActorLocation _array_element) _returnvalue)) (Variables|/Game/Systems/Blueprints/GM1/Player/Systems/Data/PDA_RocketBurst.PDA_RocketBurst_C|GetHorizontalImpulseOnly _rocketburstdata)) (Variables|/Game/Systems/Blueprints/GM1/Player/Systems/Data/PDA_RocketBurst.PDA_RocketBurst_C|GetRadialForce _rocketburstdata)) true))
      (:CastFailed
        (bind _asstatic_mesh_actor (Utilities|Casting|CastToStaticMeshActor _array_element))
        (if (Utilities|Enum|Equal(Enum) "Movable" (Variables|/Script/Engine.SceneComponent|GetMobility (Variables|/Script/Engine.StaticMeshActor|GetStaticMeshComponent _asstatic_mesh_actor)))
          (Physics|AddImpulse (Variables|/Script/Engine.StaticMeshActor|GetStaticMeshComponent _asstatic_mesh_actor) (* (Math|Vector|SelectVector (Class|KismetMathLibrary|VectorNormal2D (- (Transformation|GetActorLocation _array_element) _returnvalue) 0.0001) (Math|Vector|Normalize (- (Transformation|GetActorLocation _array_element) _returnvalue)) (Variables|/Game/Systems/Blueprints/GM1/Player/Systems/Data/PDA_RocketBurst.PDA_RocketBurst_C|GetHorizontalImpulseOnly _rocketburstdata)) (Variables|/Game/Systems/Blueprints/GM1/Player/Systems/Data/PDA_RocketBurst.PDA_RocketBurst_C|GetRadialForce _rocketburstdata)) "None" false))))))

(fn RadialStun
  (params (ignoreActors :type Array%20of%20Actor%20Object%20References) (radius :type Float%20%28double-precision%29) (duration :type Float%20%28double-precision%29))
  (bind _outactors (Collision|SphereOverlapActors (Transformation|GetActorLocation (Variables|Default|GetPlayer)) radius (Variables|Default|GetRadialLaunchChannels) "/Game/Systems/Blueprints/GM1/Player/Blueprints/BP_Player_GM1.BP_Player_GM1_C" ignoreActors))
  (for _array_element _outactors
    (Default|ApplyStun (.AsBP%20Player%20GM1 (Utilities|Casting|CastToBP_Player_GM1 _array_element)) duration)))

(fn SetFlash
  (params (Player :type BP%20Player%20GM1%20Object%20Reference) (state :type Boolean))
  (Rendering|Material|SetVectorParameterValueonMaterials (Variables|/Script/Engine.Character|GetMesh Player) "Emissive" (Math|Vector|SelectVector "1.000000,1.000000,1.000000" "0, 0, 0" state)))