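; BP_CrownSpotlight is a spotlight mesh actor for the GM1 game mode that marks the crown while it is picked up.
; BeginPlay hides the mesh, finds BP_Crown and binds its pickup and drop events to show and hide it.
; Tick moves the mesh to the tracked actor's position with a vertical offset.
; An alternative point-based mode that tracks the first-place player is present but left unhooked.
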(event Custom|BeginTracking
  (Rendering|SetVisibility (Variables|Default|GetSpotlightMesh) true false))

(event Custom|Start%20Game
  ;[1 1 1] Point-based System. To use, hook the topmost bind event into OnBeginPlay
  (EventDispatchers|BindEventtoNewFirstPlace (.AsGM%20GM1 (Utilities|Casting|CastToGM_GM1 (Game|GetGameMode))) (delegate Custom|First%20Place%20Changed)))

(event Custom|PauseTracking
  (Rendering|SetVisibility (Variables|Default|GetSpotlightMesh) false false))

(event Custom|First%20Place%20Changed
  (params (player :type BP%20Player%20GM1%20Object%20Reference))
  (bind _spotlightmesh (Variables|Default|GetSpotlightMesh))
  ;[1 1 1] Point-based System. To use, hook the topmost bind event into OnBeginPlay
  (bind _output_get (Variables|Default|SetTrackedActor player))
  ;;[0 0 0] Initial Setup
  (Utilities|FlowControl|DoOnce false
    (:Completed
      (Transformation|SetWorldLocation _spotlightmesh (Math|Vector|MakeVector (.x (Transformation|GetActorLocation _output_get)) (.y (Transformation|GetActorLocation _output_get)) (+ (.z (Transformation|GetActorLocation _output_get)) 1.25e+03)) false false)
      (Rendering|SetVisibility _spotlightmesh true false))))

(event EventBeginPlay
  ;[0 0 0] Event Bindings
  (Rendering|SetVisibility (Variables|Default|GetSpotlightMesh) false false)
  (bind _returnvalue (Actor|GetActorOfClass "/Game/Systems/Blueprints/GM1/BP_Crown.BP_Crown_C"))
  (Variables|Default|SetTrackedActor _returnvalue)
  (EventDispatchers|BindEventtoOnPickup _returnvalue (delegate Custom|BeginTracking))
  (EventDispatchers|BindEventtoOnDrop _returnvalue (delegate Custom|PauseTracking)))

(event Collision|EventActorBeginOverlap
  (params (OtherActor :type Actor%20Object%20Reference)))

(event EventTick
  (params (DeltaSeconds :type Float%20%28single-precision%29))
  (bind _trackedactor (Variables|Default|GetTrackedActor))
  (bind _returnvalue (Transformation|GetActorLocation _trackedactor))
  ;[0 0 0] Set Position
  (Utilities|IsValid _trackedactor
    (:Is%20Valid
      (Transformation|SetWorldLocation (Variables|Default|GetSpotlightMesh) (Math|Vector|MakeVector (.x _returnvalue) (.y _returnvalue) (- (.z _returnvalue) 2e+02)) false false))))

(fn ConstructionScript)