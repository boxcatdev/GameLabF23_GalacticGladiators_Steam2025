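; BP_PlayVolume defines the play area for the GM1 mode and kills any player that leaves it.
; The Radius and Height variables set the scale of its static mesh, both in the construction script and again on BeginPlay.
; When an overlapping actor exits, it casts to BP_Player_GM1 and calls HandleKill on it, ignoring all other actors.
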(event Collision|EventActorEndOverlap
  (params (OtherActor :type Actor%20Object%20Reference))
  ;[0 0 0] If a player leaves the play area, kill them
  (bind _asbp_player_gm1 (Utilities|Casting|CastToBP_Player_GM1 OtherActor))
  (Default|HandleKill _asbp_player_gm1))

(event EventBeginPlay
  (bind _radius (Variables|Default|GetRadius))
  (bind _returnvalue (/ _radius 1e+02))
  (Transformation|SetWorldScale3D (Variables|Debug|GetStaticMeshComponent) (Math|Vector|MakeVector _returnvalue _returnvalue (/ (Variables|Default|GetHeight) 2e+01))))

(fn ConstructionScript
  (bind _radius (Variables|Default|GetRadius))
  (bind _returnvalue (/ _radius 1e+02))
  (Transformation|SetWorldScale3D (Variables|Debug|GetStaticMeshComponent) (Math|Vector|MakeVector _returnvalue _returnvalue (/ (Variables|Default|GetHeight) 2e+01))))