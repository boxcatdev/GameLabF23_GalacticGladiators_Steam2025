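; BP_CollideableCrate is a crate actor with a selectable Small, Medium or Large size.
; The Size value selects one of three scale variables, which is applied to the StaticMesh as its world scale.
; The same scaling runs in both the Construction Script and BeginPlay.
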(event EventBeginPlay
  (Transformation|SetWorldScale3D (Variables|Default|GetStaticMesh) (Utilities|Select :Index (Variables|Default|GetSize) :NewEnumerator0 (Variables|Default|GetSmallSize) :NewEnumerator1 (Variables|Default|GetMediumSize) :NewEnumerator2 (Variables|Default|GetLargeSize))))

(fn ConstructionScript
  (Transformation|SetWorldScale3D (Variables|Default|GetStaticMesh) (Utilities|Select :Index (Variables|Default|GetSize) :NewEnumerator0 (Variables|Default|GetSmallSize) :NewEnumerator1 (Variables|Default|GetMediumSize) :NewEnumerator2 (Variables|Default|GetLargeSize))))